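; BP_ItemDropper spawns a configured item once a linked task actor reports that it has finished.
; On BeginPlay it binds to the task-finished event of each listed actor's BPAC_TaskActor component, printing a warning if one lacks it.
; The first completion spawns the item at the arrow's location, passes its attributes and slotable data, and calls OnSpawn.
; A flag blocks any further drops.
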(event Custom|OnTaskFinished
  (bind _itemtodrop (Variables|Default|GetItemToDrop))
  (bind _itemtodrop_2 (Variables|Default|GetItemToDrop))
  (bind (_atributes _slotable) (Utilities|Struct|BreakSt_Item _itemtodrop_2))
  (bind (_class _transformscale) (Utilities|Struct|BreakSt_Item _itemtodrop))
  (if (Variables|Default|GetdroppedAlready)
    (Development|PrintString "item already dropped")
    (else
      (bind _returnvalue (Game|SpawnActorfromClass _class (Math|Transform|MakeTransform (Transformation|GetWorldLocation (Variables|Default|GetArrow)) "0, 0, 0" _transformscale) "Undefined" "MultiplyWithRoot" 0 0))
      (bind _asbp_item_parent (Utilities|Casting|CastToBP_ItemParent _returnvalue))
      (CallFunction|SetAtributestoItem _asbp_item_parent _atributes _slotable)
      (Default|OnSpawn _asbp_item_parent)
      (Variables|Default|SetdroppedAlready true))))

(event EventBeginPlay
  (for _array_element (Variables|Default|GetTaskActors)
    (Utilities|IsValid (Actor|GetComponentbyClass _array_element "/Game/Items/BPAC_TaskActor.BPAC_TaskActor_C")
      (:Is%20Valid
        (EventDispatchers|BindEventtoOnTaskFinished (Actor|GetComponentbyClass _array_element "/Game/Items/BPAC_TaskActor.BPAC_TaskActor_C") (delegate Custom|OnTaskFinished)))
      (:Is%20Not%20Valid
        (Development|PrintString "VYBRANY ACOTR NEMA BPAC_TaskActor")))))

(fn ConstructionScript)