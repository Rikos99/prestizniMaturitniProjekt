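; Cannon actor with a widget controller for tilting and firing, showing predicted ballistic trajectories.
; Each tilt rebuilds a spline from analytic projectile height samples at the barrel's pitch.
; It also solves the high-arc angle to hit Target, printing it and drawing that path on a second spline.
; Widget firing launches a BP_CannonBall by physics velocity; an alternative, unbound shoot event moves the ball along the spline with a Timeline.
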(event Custom|shoot
  ;[1 1 1] Comment
  (bind _returnvalue (Game|SpawnActorfromClass "/Game/Items/cannon/BP_CannonBall.BP_CannonBall_C" (Transformation|GetWorldTransform (Variables|Default|GetArrow1)) "Undefined" "MultiplyWithRoot" 0 0))
  (bind _alpha (Timeline|Timeline PlayFromStart)
    (:Update
      (Transformation|SetActorLocation _returnvalue (.location (Spline|GetTransformatDistanceAlongSpline (Variables|Default|GetSpline) (Math|Float|Lerp 0.0 (Spline|GetSplineLength (Variables|Default|GetSpline)) _alpha) "World" false)) false false))))

(event Custom|CustomEvent_0
  (params (TiltStep :type Float%20%28double-precision%29))
  (bind _arrow1 (Variables|Default|GetArrow1))
  (bind _target (Variables|Default|GetTarget))
  (bind _returnvalue (Transformation|GetWorldLocation _arrow1))
  (bind _arrow (Variables|/Game/Items/cannon/BP_Basket.BP_Basket_C|GetArrow _target))
  (bind _returnvalue_2 (Transformation|GetWorldLocation _arrow))
  ;[1 1 1] nakloneni kanonu
  (Utilities|FlowControl|Sequence
    (:then_0
      (Transformation|AddLocalRotation (Variables|Default|GetCylinder) (Math|Rotator|MakeRotator 0.0 TiltStep 0.0) false false)
      ;[1 1 1] vypocitam po metrech body pro vytvoreni krivky letu
      (bind _newsplinepoints (CallFunction|GetSplinePoints (+ (.pitch (Transformation|GetWorldRotation (Variables|Default|GetCylinder))) 9e+01)))
      ;[1 1 1] setnu body krivky
      (Spline|SetSplinePoints (Variables|Default|GetSpline) _newsplinepoints "World" true))
    (:then_1
      (bind _uhel (CallFunction|VypocitejUhel (/ (Math|Float|Absolute(Float) (- (.x _returnvalue_2) (.x _returnvalue))) 1e+02) (Variables|Default|GetPocatecniRychlostGlob) (Variables|Default|GetgravitacniSilaGlob) (/ (- (.z _returnvalue_2) (.z _returnvalue)) 1e+02)))
      (Development|PrintString (Utilities|String|ToString(Float) _uhel) true true "(R=1.000000,G=0.300146,B=0.000000,A=1.000000)")
      (Rendering|Debug|DrawDebugLine (Transformation|GetWorldLocation _arrow) (Transformation|GetWorldLocation _arrow1) "(R=1.000000,G=0.000000,B=0.096653,A=1.000000)" 2.0 1.0)
      (bind _newsplinepoints_2 (CallFunction|GetSplinePoints _uhel))
      (Spline|SetSplinePoints (Variables|Default|GetSpline1) _newsplinepoints_2 "World" true))))

(event Custom|shootReal
  (bind _returnvalue (Game|SpawnActorfromClass "/Game/Items/cannon/BP_CannonBall.BP_CannonBall_C" (Transformation|GetWorldTransform (Variables|Default|GetArrow1)) "Undefined" "MultiplyWithRoot" 0 0))
  (Physics|SetPhysicsLinearVelocity (Variables|/Game/Items/cannon/BP_CannonBall.BP_CannonBall_C|GetSphere _returnvalue) (* (Math|Vector|GetForwardVector (Variables|/Game/Items/cannon/BP_CannonBall.BP_CannonBall_C|GetSphere _returnvalue)) (* (Variables|Default|GetPocatecniRychlostGlob) 1e+02)) false "None"))

(event EventBeginPlay
  (bind _returnvalue (UserInterface|CreateWidget "/Game/Items/cannon/UI/WBP_CannonController.WBP_CannonController_C" (Game|GetPlayerController 0)))
  (EventDispatchers|BindEventtoTiltCannon _returnvalue (delegate Custom|CustomEvent_0))
  (EventDispatchers|BindEventtoSHOOT _returnvalue (delegate Custom|shootReal))
  (UserInterface|SetWidget (Variables|Default|GetWidget) _returnvalue))

(event EventInteract
  (params (inventory :type BPAC%20Inventory%20Object%20Reference) (hitComponent :type Primitive%20Component%20Object%20Reference)))

(fn ConstructionScript)

(fn RotateCylinder
  (Transformation|AddLocalRotation (Variables|Default|GetCylinder) "-0.500000,0.000000,0.000000" false false))

(fn GetSplinePoints
  (params (angle :type Float%20%28double-precision%29))
  (for _index (range 0 20)
    (bind _vyska (CallFunction|VypocitejVysku (Math|Conversions|ToFloat(Integer) _index) (Variables|Default|GetPocatecniRychlostGlob) angle (Variables|Default|GetgravitacniSilaGlob)))
    (Utilities|Array|Add (LocalVariables|Getpoints) (+ (Transformation|GetWorldLocation (Variables|Default|GetSpline)) (* "0.000000,0.000000,1.000000" (* _vyska 1e+02)) (* (* _index 100) (Math|Vector|GetForwardVector (Variables|Default|GetDefaultSceneRoot))))))
  (return (LocalVariables|Getpoints)))

(fn VypocitejVysku
  (params (vzdalenost :type Float%20%28double-precision%29) (pocatecniRychlost :type Float%20%28double-precision%29) (Uhel :type Float%20%28double-precision%29) (GravitacniSila :type Float%20%28double-precision%29))
  (return (- (* vzdalenost (Math|Trig|Tan(Degrees) Uhel)) (/ (* GravitacniSila (Math|Float|Square vzdalenost)) (* (Math|Float|Square pocatecniRychlost) (Math|Float|Square (Math|Trig|Cos(Degrees) Uhel)) 2.0)))))

(fn VypocitejUhel
  (params (vzdalenost :type Float%20%28double-precision%29) (pocatecniRychlost :type Float%20%28double-precision%29) (GravitacniSila :type Float%20%28double-precision%29) (vyska :type Float%20%28double-precision%29))
  (bind _output_get (LocalVariables|Setdiskriminant (- (Math|Float|Square vzdalenost) (* 4.0 (/ (* GravitacniSila (Math|Float|Square vzdalenost)) (* (Math|Float|Square pocatecniRychlost) 2.0)) (+ vyska (/ (* GravitacniSila (Math|Float|Square vzdalenost)) (* (Math|Float|Square pocatecniRychlost) 2.0)))))))
  (if (>= _output_get 0.0)
    (return (Class|KismetMathLibrary|DegAtan (/ (+ vzdalenost (Math|Float|Sqrt (LocalVariables|Getdiskriminant))) (* (/ (* GravitacniSila (Math|Float|Square vzdalenost)) (* (Math|Float|Square pocatecniRychlost) 2.0)) 2.0))))
    (else
      (Development|PrintString "UHEL NEZLE VYPOCITAT"))))