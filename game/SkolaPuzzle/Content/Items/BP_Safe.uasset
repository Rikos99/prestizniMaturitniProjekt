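; BP_Safe is an interactable safe with three keyholes and a handle (Klika) that checks inserted keys.
; Using an allowed slotable item on a keyhole spawns it attached there, removes it from inventory and copies its attributes over.
; The handle compares each stored item's KeyValue attribute to the safe's, accumulating CorrectKeys without resetting it.
; If that count equals the map's entry count, Opened is set; opening itself is only a debug print.
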(event EventInteract
  (params (inventory :type BPAC%20Inventory%20Object%20Reference) (hitComponent :type Primitive%20Component%20Object%20Reference))
  (if (Utilities|Array|ContainsItem (Variables|Default|GetSlots) hitComponent)
    (CallFunction|OnInteractKeyhole inventory hitComponent)
    (elif (== hitComponent (Variables|Default|Getklika))
      (if (not (Variables|Default|GetOpened))
        (CallFunction|OnInteractKlika)))))

(event EventBeginPlay
  (Variables|Default|SetSlots (Utilities|Array|MakeArray (Variables|Default|GetKlicovaDirka1) (Variables|Default|GetKlicovaDirka2) (Variables|Default|GetKlicovaDirka3)))
  (Variables|Default|SetItemsInSlots (Utilities|Map|MakeMap 0 0 1 0 2 0)))

(fn ConstructionScript)

(fn OnInteractKeyhole
  (params (inventory :type BPAC%20Inventory%20Object%20Reference) (hitComponent :type Primitive%20Component%20Object%20Reference))
  (bind _inventorymap (Variables|/Game/Player/BPAC_Inventory.BPAC_Inventory_C|GetInventoryMap inventory))
  (bind _activeslotindex (Variables|/Game/Player/BPAC_Inventory.BPAC_Inventory_C|GetActiveSlotIndex inventory))
  (bind _slots (Variables|Default|GetSlots))
  (bind _value (Utilities|Map|Find _inventorymap _activeslotindex))
  (bind (_objectname _slotimage _class _atributes _transformscale _slotable) (Utilities|Struct|BreakSt_Item _value))
  (bind (_objectname_2 _slotimage_2 _class_2 _atributes_2 _transformscale_2) (Utilities|Struct|BreakSt_Item _value))
  (if _slotable
    (if (!= (Utilities|Array|FindItem (Variables|Default|GetSlotableItems) _class) -1)
      (if (Utilities|ClassIsChildOf _class_2 "/Game/Items/BP_ItemParent.BP_ItemParent_C")
        (bind _returnvalue (Game|SpawnActorfromClass _class_2 (Math|Transform|MakeTransform (+ (Transformation|GetWorldLocation (Utilities|Array|Get(acopy) _slots (Utilities|Array|FindItem _slots hitComponent))) (* (Transformation|GetActorForwardVector) 1e+01)) (Math|Conversions|RotationFromXVector (* (Transformation|GetActorForwardVector) -1.0)) _transformscale_2) "AlwaysSpawn" "MultiplyWithRoot" 0 0))
        (bind _asbp_item_parent (Utilities|Casting|CastToBP_ItemParent _returnvalue))
        (Utilities|Map|Add (Variables|Default|GetItemsInSlots) (Utilities|Array|FindItem (Variables|Default|GetSlots) hitComponent) _asbp_item_parent)
        (Utilities|FlowControl|Sequence
          (:then_0
            (bind _returnvalue_2 (Transformation|AttachComponentToComponent _asbp_item_parent hitComponent "" "SnapToTarget" "SnapToTarget" "KeepWorld" true))
            (Class|BPIDisablePhysics|DisablePhysics(Message) _returnvalue)
            (Development|PrintString (Utilities|String|ToString(Boolean) _returnvalue_2)))
          (:then_1
            (bind _removeditemstruct (Default|RemoveItem inventory (Variables|/Game/Player/BPAC_Inventory.BPAC_Inventory_C|GetActiveSlotIndex inventory)))
            (Default|SetAtributesfromStructtoObject inventory _asbp_item_parent (.Atributes (Utilities|Struct|BreakSt_Item _removeditemstruct)) (.Slotable (Utilities|Struct|BreakSt_Item _removeditemstruct)))))))))

(fn OnInteractKlika
  (bind _itemsinslots (Variables|Default|GetItemsInSlots))
  (bind _keys (Utilities|Map|Keys _itemsinslots))
  (for _array_element _keys
    (if (.ReturnValue (Utilities|Map|Find _itemsinslots _array_element))
      (if (Utilities|IsValid (.Value (Utilities|Map|Find _itemsinslots _array_element)))
        (if (.ReturnValue (Utilities|Map|Find (Variables|/Game/Items/BP_ItemParent.BP_ItemParent_C|GetItemAtributes (.Value (Utilities|Map|Find _itemsinslots _array_element))) "KeyValue"))
          (if (Utilities|Enum|Equal(Enum) (Variables|Default|GetKeyValue) (.Value (Utilities|Map|Find (Variables|/Game/Items/BP_ItemParent.BP_ItemParent_C|GetItemAtributes (.Value (Utilities|Map|Find _itemsinslots _array_element))) "KeyValue")))
            (Math|Integer|IncrementInt (LocalVariables|GetcorrectKeys)))))
      (else
        (Development|PrintString "nenasel se slot" true true "(R=1.000000,G=0.034640,B=0.000000,A=1.000000)"))))
  (if (== (LocalVariables|GetcorrectKeys) (Utilities|Array|Length _keys))
    (Variables|Default|SetOpened true)
    (Development|PrintString "OTEVRIT DVERE")
    (else
      (Development|PrintString "NEPODARILO SE OTEVRIT DVERE"))))