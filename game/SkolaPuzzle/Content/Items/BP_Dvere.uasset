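; Interactable door that swings open or closed when unlocked; a successful OnLockUsed event unlocks it.
; Interact, gated by IsOpening, chains timelines that turn the handle, yaw the root from its current world rotation and return the handle.
; When locked with a handle, it shows a data-table line through BPDialogueComponent while handle and door rattle.
; The construction script applies configurable meshes, toggles handle visibility and adds an optional clear or foggy window.
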(event EventBeginPlay)

(event Collision|EventActorBeginOverlap
  (params (OtherActor :type Actor%20Object%20Reference)))

(event EventTick
  (params (DeltaSeconds :type Float%20%28single-precision%29)))

(event EventInteract
  (params (inventory :type BPAC%20Inventory%20Object%20Reference) (hitComponent :type Primitive%20Component%20Object%20Reference))
  (bind _bp_dialoguecomponent (Variables|Default|GetBP_DialogueComponent))
  (if (not (Variables|Default|GetIsOpening))
    (Variables|Default|SetIsOpening true)
    (if (Variables|Default|GetUnlocked)
      ;[0.07812 0 0] Open/Close whole doors
      (bind _rotate_door_handle (Timeline|TimelineRotateDoorHandle PlayFromStart)
        (:Update
          (Transformation|SetRelativeRotation (Variables|Default|Getdvere_Dvere_Zamek_Klika) (Math|Rotator|MakeRotator 0.0 _rotate_door_handle 0.0) false false))
        (:Finished
          (Utilities|FlowControl|Sequence
            (:then_0
              (Variables|Default|SetCurrentWorldRotationZ (.yaw (Transformation|GetWorldRotation (Variables|Default|GetDefaultSceneRoot))))
              (if (Variables|Default|GetClosed)
                (bind _open (Timeline|TimelineOpenDoor PlayFromStart)
                  (:Update
                    (Transformation|SetRelativeRotation (Variables|Default|GetDefaultSceneRoot) (Math|Rotator|MakeRotator 0.0 0.0 (+ _open (Variables|Default|GetCurrentWorldRotationZ))) false false))
                  (:Finished
                    (Variables|Default|SetClosed false)))
                (else
                  (bind _close (Timeline|TimelineCloseDoor PlayFromStart)
                    (:Update
                      (Transformation|SetRelativeRotation (Variables|Default|GetDefaultSceneRoot) (Math|Rotator|MakeRotator 0.0 0.0 (+ _close (Variables|Default|GetCurrentWorldRotationZ))) false false))
                    (:Finished
                      (Variables|Default|SetClosed true))))))
            (:then_1
              (bind _rotate_back (Timeline|RotateDoorHandleBack PlayFromStart)
                (:Update
                  (Transformation|SetRelativeRotation (Variables|Default|Getdvere_Dvere_Zamek_Klika) (Math|Rotator|MakeRotator 0.0 _rotate_back 0.0) false false))
                (:Finished
                  (Variables|Default|SetIsOpening false)))))))
      (elif (Variables|Default|GetDoorHandle)
        (Utilities|FlowControl|Sequence
          (:then_0
            ;[1 0.5249 0.8248] Set Text
            (if (!= (Variables|Default|GetHlaska%20Row%20Name) "")
              _
              (else
                (bind _output_get (Variables|Default|SetHlaska%20Row%20Name "Dvere"))))
            (Default|SetNewVariables _bp_dialoguecomponent _output_get "/Game/UI/Dialogue/Hlasky_DataTable.Hlasky_DataTable" false "" 0 "NewEnumerator5")
            (Default|Interact _bp_dialoguecomponent))
          (:then_1
            ;[1 0.8747 0.3581] Rotate Door Handle
            (bind _rattle_door_handle (Timeline|RotateDoorHandleLocked PlayFromStart)
              (:Update
                (Transformation|SetRelativeRotation (Variables|Default|Getdvere_Dvere_Zamek_Klika) (Math|Rotator|MakeRotator 0.0 _rattle_door_handle 0.0) false false))))
          (:then_2
            ;[1 0.8747 0.3581] Rattle Doors
            (Variables|Default|SetCurrentWorldRotationZ (.yaw (Transformation|GetWorldRotation (Variables|Default|GetDefaultSceneRoot))))
            (bind _rattledoors (Timeline|Timeline_RattleWholeDoors PlayFromStart)
              (:Update
                (if (Variables|Default|GetClosed)
                  (Variables|Default|SetRattle%20Doors _rattledoors)
                  (else
                    (bind _output_get_2 (Variables|Default|SetRattle%20Doors (* _rattledoors -1.0)))))
                (Transformation|SetRelativeRotation (Variables|Default|GetDefaultSceneRoot) (Math|Rotator|MakeRotator 0.0 0.0 (+ _output_get_2 (Variables|Default|GetCurrentWorldRotationZ))) false false))
              (:Finished
                (bind _rotate_back_2 (Timeline|RotateDoorHandleBackLocked PlayFromStart)
                  (:Update
                    (Transformation|SetRelativeRotation (Variables|Default|Getdvere_Dvere_Zamek_Klika) (Math|Rotator|MakeRotator 0.0 _rotate_back_2 0.0) false false))
                  (:Finished
                    (Variables|Default|SetIsOpening false)))))))))))

(event EventOnLockUsed
  (params (successful :type Boolean))
  (if successful
    (Variables|Default|SetUnlocked true)))

(fn ConstructionScript
  ;[0.15 0.15 0.15 0.5] Set models from parameters
  (Components|StaticMesh|SetStaticMesh (Variables|Default|Getdvere_Dvere) (Variables|Default|GetDoorMesh))
  (Components|StaticMesh|SetStaticMesh (Variables|Default|Getdvere_Dvere_Zamek_Base) (Variables|Default|GetDoorHandleBaseMesh))
  (Components|StaticMesh|SetStaticMesh (Variables|Default|Getdvere_Dvere_Zamek_Klika) (Variables|Default|GetDoorHandleMesh))
  ;[0.15 0.15 0.15 0.5] Enable/Disable door handle
  (if (Variables|Default|GetDoorHandle)
    _
    (else
      (Rendering|ToggleVisibility (Variables|Default|Getdvere_Dvere_Zamek_Base) true)
      (Rendering|ToggleVisibility (Variables|Default|Getdvere_Dvere_Zamek_Klika) false)))
  ;[0.15 0.15 0.15 0.5] Enable/Disable Window
  (if (Variables|Default|GetOkno)
    (bind _returnvalue (AddComponent|AddStaticMeshComponent false))
    (if (Variables|Default|GetFoggy%20Window)
      (Rendering|Material|SetMaterial _returnvalue 0 "/Game/Materials/MI_DvereServerovnaOknoFoggy.MI_DvereServerovnaOknoFoggy")
      (else
        (Rendering|Material|SetMaterial _returnvalue 0 "/Game/Materials/MI_DvereServerovnaOknoClear.MI_DvereServerovnaOknoClear")))))