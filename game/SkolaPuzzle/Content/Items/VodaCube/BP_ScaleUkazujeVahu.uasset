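; Weighing scale item that shows the total mass of cubes placed in its three box slots on a widget display.
; Items of slotable classes enter by overlapping a box or by being dropped from the Inventory on Interact; BindCube records and attaches them, disabling cube physics.
; OnWeightChanged adds or, on slot removal, subtracts density from DT_CubeMaterials times the cube's volume, then updates the Czech kilogram readout.
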(event Custom|BoxColliderOnBeginOverlap
  (params (OverlappedComponent :type Primitive%20Component%20Object%20Reference) (OtherActor :type Actor%20Object%20Reference) (OtherComp :type Primitive%20Component%20Object%20Reference) (OtherBodyIndex :type Integer) (bFromSweep :type Boolean) (SweepResult :type Hit%20Result%20Structure%20%28by%20ref%29))
  (if (Utilities|Array|ContainsItem (Variables|Default|GetSlotableItems) (Utilities|GetClass OtherActor))
    (bind _asbp_item_parent (Utilities|Casting|CastToBP_ItemParent OtherActor))
    (CallFunction|BindCube _asbp_item_parent OverlappedComponent)))

(event EventInteract
  (params (inventory :type BPAC%20Inventory%20Object%20Reference) (hitComponent :type Primitive%20Component%20Object%20Reference))
  (CallFunction|OnInteract inventory hitComponent))

(event EventBeginPlay
  (Utilities|FlowControl|Sequence
    (:then_0
      (bind _returnvalue (UserInterface|CreateWidget "/Game/Items/VodaCube/WBP_ScaleInterface.WBP_ScaleInterface_C"))
      (bind _output_get (Variables|Default|SetScaleWidget _returnvalue))
      (UserInterface|SetWidget (Variables|Default|GetWidgetComponent) _output_get))
    (:then_1
      (Variables|Default|SetItemsInSlots (Utilities|Map|MakeMap 0 0 1 0 2 0)))
    (:then_2
      (bind _output_get_2 (Variables|Default|SetSlots (Utilities|Array|MakeArray (Variables|Default|GetBox1) (Variables|Default|GetBox2) (Variables|Default|GetBox3))))
      (for _array_element _output_get_2
        (bind _asbox_collision (Utilities|Casting|CastToBoxComponent _array_element)
          (:then
            (Collision|BindEventtoOnComponentBeginOverlap _asbox_collision (delegate Custom|BoxColliderOnBeginOverlap)))
          (:CastFailed
            (Development|PrintString "cast to boxcompoent failed in bp_scale event graph")))))))

(fn ConstructionScript)

(fn OnInteract
  (params (inventory :type BPAC%20Inventory%20Object%20Reference) (hitComponent :type Primitive%20Component%20Object%20Reference%20%28by%20ref%29))
  (bind (_origin _boxextent) (Collision|GetComponentBounds hitComponent))
  (bind _returnvalue (Transformation|GetWorldLocation hitComponent))
  (Utilities|FlowControl|Sequence
    (:then_0
      (if (not (Utilities|Array|ContainsItem (Variables|Default|GetSlots) hitComponent))
        (return)))
    (:then_1
      (bind _class (Default|GetClassOfIteminHand inventory))
      (if (not (Utilities|Array|ContainsItem (Variables|Default|GetSlotableItems) _class))
        (return)))
    (:then_2
      (bind (_itemdropped _actorref) (Default|DropItem inventory (Math|Vector|MakeVector (.x _returnvalue) (.y _returnvalue) (+ (.z _origin) (.z _boxextent)))))
      (if _itemdropped
        (CallFunction|BindCube _actorref hitComponent)
        (else
          (return))))))

(fn OnWeightChanged
  (params (cubeActor :type BP%20Cube%20Object%20Reference) (weightAdded :type Boolean))
  (bind _itematributes (Variables|/Game/Items/BP_ItemParent.BP_ItemParent_C|GetItemAtributes cubeActor))
  (bind _returnvalue (Utilities|GetDataTableRow "/Game/Items/VodaCube/DT_CubeMaterials.DT_CubeMaterials" (Utilities|String|StringToName (.Value (Utilities|Map|Find _itematributes "CubeMaterialsDataTableRowName"))))
    (:then
      (bind _output_get (Variables|Default|SetWeight (+ (Variables|Default|GetWeight) (* (* (.density _returnvalue) (.Value (Utilities|Map|Find _itematributes "volume"))) (Math|Float|SelectFloat 1.0 -1.0 weightAdded)))))
      (Default|ChangeText (Variables|Default|GetScaleWidget) (Utilities|Text|ToText(String) (Utilities|String|Append "Aktuánlí váha: " (Utilities|String|ToString(Float) _output_get) "kg"))))))

(fn RemoveSlottedItem
  (params (object :type BP%20Item%20Parent%20Object%20Reference) (slotIndex :type Integer))
  (bind _asbp_cube (Utilities|Casting|CastToBP_Cube object)
    (:then
      (CallFunction|OnWeightChanged _asbp_cube false)
      (|CallParentFunction object slotIndex))
    (:CastFailed
      (Development|PrintString "cast to bP-cube failed in bp-scale (removeSlottedItem)"))))

(fn BindCube
  (params (item :type BP%20Item%20Parent%20Object%20Reference) (VahaComponent :type Primitive%20Component%20Object%20Reference))
  (bind _values (Utilities|Map|Values (Variables|Default|GetItemsInSlots)))
  (if (not (Utilities|Array|ContainsItem _values item))
    (Utilities|FlowControl|Sequence
      (:then_0
        (Utilities|Map|Add (Variables|Default|GetItemsInSlots) (Utilities|Array|FindItem (Variables|Default|GetSlots) VahaComponent) item))
      (:then_2
        (bind _asbp_cube (Utilities|Casting|CastToBP_Cube item)
          (:then
            (CallFunction|OnWeightChanged _asbp_cube true)
            (Physics|SetSimulatePhysics (Variables|/Game/Items/VodaCube/BP_Cube.BP_Cube_C|GetStaticMesh _asbp_cube) false))
          (:CastFailed
            (Development|PrintString "cast to bp_cube in bp-scale (onInteract)"))))
      (:then_3
        (Transformation|AttachComponentToComponent item VahaComponent "None" "SnapToTarget" "KeepRelative" "KeepRelative" true)))))