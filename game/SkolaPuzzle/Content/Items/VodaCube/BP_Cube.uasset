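; BP_Cube is a cube item whose material, mass and size are driven by its string attribute map, ItemAtributes.
; The construction script runs OnSpawn, which looks up DT_CubeMaterials to set the visual material and override mass from density and linear scale.
; It also applies any scale attribute to the mesh and writes the cubed value back as volume.
; BeginPlay and DisablePhysics are empty.
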(event EventBeginPlay)

(fn ConstructionScript
  (CallFunction|OnSpawn))

(fn OnSpawn
  (bind _itematributes (Variables|Default|GetItemAtributes))
  (bind (_value _returnvalue) (Utilities|Map|Find _itematributes "scale"))
  (bind _returnvalue_2 (Math|Conversions|ToFloat(Integer) _value))
  (Utilities|FlowControl|Sequence
    (:then_0
      (Variables|Default|SetMainStaticMesh (Variables|Default|GetStaticMesh)))
    (:then_1
      (bind _returnvalue_3 (Utilities|GetDataTableRow "/Game/DataTables/DT_CubeMaterials.DT_CubeMaterials" (Utilities|String|StringToName (.Value (Utilities|Map|Find (Variables|Default|GetItemAtributes) "CubeMaterialsDataTableRowName"))))
        (:then
          (Utilities|FlowControl|Sequence
            (:then_0
              (Rendering|Material|SetMaterial (Variables|Default|GetStaticMesh) 0 (.visualmeterial _returnvalue_3)))
            (:then_1
              (Class|PrimitiveComponent|SetMassOverrideinKg (Variables|Default|GetStaticMesh) "None" (* (.density _returnvalue_3) (/ (Math|Conversions|ToFloat(Integer) (.Value (Utilities|Map|Find (Variables|Default|GetItemAtributes) "scale"))) 1e+02)) true))))))
    (:then_2
      (if _returnvalue
        (Transformation|SetWorldScale3D (Variables|Default|GetStaticMesh) (Math|Conversions|ToVector(Float) _returnvalue_2))
        (Utilities|Map|Add (Variables|Default|GetItemAtributes) "volume" (Utilities|String|ToString(Float) (Math|Float|Power _returnvalue_2 3.0)))))))

(fn DisablePhysics)