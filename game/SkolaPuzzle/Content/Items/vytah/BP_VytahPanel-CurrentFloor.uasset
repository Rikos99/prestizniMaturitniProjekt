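; Elevator (vytah) panel actor that shows the current floor number on a text display, initialized from FloorNumber in the construction script.
; ChangeFloorNum loops over the floors between current and target, passing each to ChangeText.
; Both loops ascend with no delay, so only the higher floor remains displayed, even when the target is lower.
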(event Custom|Change%20Floor%20Num
  (params (Current%20Floor :type Integer) (Target%20Floor :type Integer))
  (if (not (== Current%20Floor Target%20Floor))
    (if (> Current%20Floor Target%20Floor)
      (for _index (range Target%20Floor Current%20Floor)
        (CallFunction|ChangeText _index))
      (else
        (for _index_2 (range Current%20Floor Target%20Floor)
          (CallFunction|ChangeText _index_2))))))

(event EventBeginPlay)

(event Collision|EventActorBeginOverlap
  (params (OtherActor :type Actor%20Object%20Reference)))

(event EventTick
  (params (DeltaSeconds :type Float%20%28single-precision%29)))

(fn ConstructionScript
  (Rendering|Components|TextRender|SetText (Variables|Default|GetVytahPanelDisplay) (Variables|Default|GetFloor%20Number)))

(fn ChangeText
  (params (Floor :type Integer))
  (Rendering|Components|TextRender|SetText (Variables|Default|GetVytahPanelDisplay) (Utilities|Text|ToText(Integer) Floor)))