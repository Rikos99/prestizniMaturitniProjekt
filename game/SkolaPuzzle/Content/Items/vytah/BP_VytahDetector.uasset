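; BP_VytahDetector is an elevator ("vytah") detector actor that reacts when the player pawn stops overlapping it.
; After a five-second delay, it finds the BP_VytahDvere door actor by class and closes the doors.
; It then changes the floor level, described as the display number, to a hardcoded floor 8 unless that is already current.
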(event EventBeginPlay)

(event Collision|EventActorBeginOverlap
  (params (OtherActor :type Actor%20Object%20Reference)))

(event EventTick
  (params (DeltaSeconds :type Float%20%28single-precision%29)))

(event Collision|EventActorEndOverlap
  (params (OtherActor :type Actor%20Object%20Reference))
  (if (== OtherActor (Game|Player|GetPlayerPawn 0))
    (Utilities|FlowControl|Delay 5.0)
    ;[0.15 0.15 0.15 0.5] Close doors
    (bind _returnvalue (Actor|GetActorOfClass "/Game/Items/vytah/BP_VytahDvere.BP_VytahDvere_C"))
    (Default|CloseDoors _returnvalue)
    ;[0.15 0.15 0.15 0.5] Change number on display
    (bind _current_level (CallFunction|GetCurrentFloorLevel))
    (if (not (== _current_level 8))
      (CallFunction|ChangeFloorLevel self _current_level 8))))

(fn ConstructionScript)