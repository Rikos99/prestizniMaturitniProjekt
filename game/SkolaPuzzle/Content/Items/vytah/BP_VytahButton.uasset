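; Interactable elevator call button that nudges inward briefly when its button or base mesh is used.
; It prints the current floor level and, unless that is 8, calls ChangeFloorLevel from hard-coded floor 8 to that level.
; After a delay scaled by the floor difference, plus a fixed margin, it opens the first BP_VytahDvere doors found in the level.
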(event EventBeginPlay)

(event Collision|EventActorBeginOverlap
  (params (OtherActor :type Actor%20Object%20Reference)))

(event EventTick
  (params (DeltaSeconds :type Float%20%28single-precision%29)))

(event EventInteract
  (params (inventory :type BPAC%20Inventory%20Object%20Reference) (hitComponent :type Primitive%20Component%20Object%20Reference))
  (bind _patro1_chodbakratka_vytah_tlacitko_vytah_tlacitko_button (Variables|Default|Getpatro1-chodbaKratka-vytah-tlacitko_Vytah_Tlacitko_Button))
  (if (or (== hitComponent (Variables|Default|Getpatro1-chodbaKratka-vytah-tlacitko_Vytah_Tlacitko_Button)) (== hitComponent (Variables|Default|Getpatro1-chodbaKratka-vytah-tlacitko_Vytah_Tlacitko_Base)))
    (Transformation|AddLocalOffset _patro1_chodbakratka_vytah_tlacitko_vytah_tlacitko_button "-2.500000,0.000000,0.000000" false false)
    (Utilities|FlowControl|Delay 0.2)
    (Transformation|AddLocalOffset _patro1_chodbakratka_vytah_tlacitko_vytah_tlacitko_button "2.500000,0.000000,0.000000" false false)
    (bind _current_level (CallFunction|GetCurrentFloorLevel))
    (Development|PrintString (Utilities|String|ToString(Integer) _current_level))
    (if (== _current_level 8)
      _
      (else
        (CallFunction|ChangeFloorLevel self 8 _current_level)))
    (Utilities|FlowControl|Delay (Math|Conversions|ToFloat(Integer) (+ (* (- 8 _current_level) 5) 2)))
    (bind _returnvalue (Actor|GetActorOfClass "/Game/Items/vytah/BP_VytahDvere.BP_VytahDvere_C"))
    (Default|OpenDoors _returnvalue)))

(fn ConstructionScript)