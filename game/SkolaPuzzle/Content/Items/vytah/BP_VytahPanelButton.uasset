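; Elevator panel button that either opens the elevator doors or sends the player to another floor's level, showing a decal or floor number accordingly.
; On Interact, a floor button compares the current floor with the target level name's last digit, closes the doors and starts the panel's floor display.
; After a delay scaled by floors travelled, it saves player position, rotation and inventory to the GameInstance, then opens the level.
; Item saving is disconnected.
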(event EventBeginPlay)

(event Collision|EventActorBeginOverlap
  (params (OtherActor :type Actor%20Object%20Reference)))

(event EventTick
  (params (DeltaSeconds :type Float%20%28single-precision%29)))

(event EventInteract
  (params (inventory :type BPAC%20Inventory%20Object%20Reference) (hitComponent :type Primitive%20Component%20Object%20Reference))
  (bind _target_level (Variables|Default|GetTarget%20Level))
  (bind _returnvalue (Utilities|ToString(SoftObjectReference) _target_level))
  (bind _returnvalue_2 (Utilities|String|Right _returnvalue 1))
  (bind _returnvalue_3 (Math|Conversions|ToInteger(Byte) _returnvalue_2))
  (if (not (Variables|Default|GetOtevrit%20Dvere))
    (bind _current_level (CallFunction|GetCurrentFloorLevel))
    (if (and (Utilities|IsValidSoftObjectReference _target_level) (!= _current_level _returnvalue_3))
      (Variables|Default|SetFrom _current_level)
      (Variables|Default|SetTo _returnvalue_3)
      (bind _returnvalue_4 (Actor|GetActorOfClass "/Game/Items/vytah/BP_VytahDvere.BP_VytahDvere_C"))
      (Utilities|FlowControl|Sequence
        (:then_0
          (Default|CloseDoors _returnvalue_4))
        (:then_1
          (bind _returnvalue_5 (Actor|GetActorOfClass "/Game/Items/vytah/BP_VytahPanel.BP_VytahPanel_C"))
          (Default|ChangeFloorNum _returnvalue_5 (Variables|Default|GetFrom) (Variables|Default|GetTo))
          (Utilities|FlowControl|Delay (* (Math|Integer|Absolute(Integer) (- (Variables|Default|GetFrom) (Variables|Default|GetTo))) 5.0))
          (Utilities|Time|ClearandInvalidateTimerbyHandle (Variables|/Game/Items/vytah/BP_VytahPanel.BP_VytahPanel_C|GetDisplay%20Timer _returnvalue_5))
          (bind _asbp_first_person_character (Utilities|Casting|CastToBP_FirstPersonCharacter (Game|Player|GetPlayerPawn 0)))
          (bind _asbp_game_instance (Utilities|Casting|CastToBP_GameInstance (Game|GetGameInstance)))
          (Utilities|FlowControl|Sequence
            (:then_0
              (CallFunction|SavePlayerTransform _asbp_first_person_character _asbp_game_instance))
            (:then_1
              (CallFunction|SavePlayerInventory _asbp_first_person_character _asbp_game_instance))
            (:then_3
              (Game|OpenLevel(byObjectReference) (Variables|Default|GetTarget%20Level)))))))
    (else
      (bind _returnvalue_6 (Actor|GetActorOfClass "/Game/Items/vytah/BP_VytahDvere.BP_VytahDvere_C"))
      (Default|OpenDoors _returnvalue_6))))

(fn ConstructionScript
  (bind _textrender (Variables|Default|GetTextRender))
  (if (Variables|Default|GetOtevrit%20Dvere)
    (Rendering|SetVisibility _textrender false false)
    (else
      (Rendering|SetVisibility (Variables|Default|GetDecal) false false)
      (Rendering|Components|TextRender|SetText _textrender (Variables|Default|GetFloor%20Number)))))

(fn SavePlayerTransform
  (params (firstPersonCharacter :type BP%20First%20Person%20Character%20Object%20Reference) (gameInstance :type BP%20Game%20Instance%20Object%20Reference))
  (Variables|/Game/BP_GameInstance.BP_GameInstance_C|SetPlayerPos gameInstance (Transformation|GetWorldLocation (Variables|/Script/Engine.Actor|GetRootComponent firstPersonCharacter)))
  (Variables|/Game/BP_GameInstance.BP_GameInstance_C|SetCameraRotation gameInstance (Transformation|GetActorRotation (Game|GetPlayerController 0))))

(fn SaveItems
  (params (gameInstance :type BP%20Game%20Instance%20Object%20Reference)))

(fn SavePlayerInventory
  (params (firstPersonCharacter :type BP%20First%20Person%20Character%20Object%20Reference) (gameInstance :type BP%20Game%20Instance%20Object%20Reference))
  (Variables|/Game/BP_GameInstance.BP_GameInstance_C|SetPlayerInventory gameInstance (Variables|/Game/Player/BPAC_Inventory.BPAC_Inventory_C|GetInventoryMap (Variables|/Game/Player/BP_FirstPersonCharacter.BP_FirstPersonCharacter_C|GetBPAC_Inventory firstPersonCharacter))))