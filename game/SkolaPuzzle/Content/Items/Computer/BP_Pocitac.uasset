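; Interactable PC (Pocitac) that lets the player plug slotable inventory items, currently USB flash disks, into its USB sockets.
; Interacting with the USB hitbox checks the active inventory item, then looks for empty entries in the slot map.
; The item is spawned, attached to a numbered mesh socket with physics off, given its stored attributes, and removed from the inventory.
; An older flash-disk-only version remains as unreachable nodes.
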(event Custom|IDKpc
  (params (inventory :type BPAC%20Inventory%20Object%20Reference) (hitComponent :type Primitive%20Component%20Object%20Reference))
  ;[1 1 1] Comment
)

(event EventInteract
  (params (inventory :type BPAC%20Inventory%20Object%20Reference) (hitComponent :type Primitive%20Component%20Object%20Reference))
  (bind _pcstaticmesh (Variables|Default|GetPcStaticMesh))
  (bind _returnvalue (Transformation|GetWorldRotation _pcstaticmesh))
  ;[1 1 1] jaky component pocitace jsem raycastem trefili (kdyby se potom mely pridat dalsi casti, jako power button, popripade jine porty)
  (bind _output_get (Variables|Default|SetInventory inventory))
  (if (== hitComponent (Variables|Default|GetusbHitbox))
    ;[1 1 1] jestli hrac v ruce drzi usb lfash disk
    (if (.slotable (.Value (Utilities|Map|Find (Variables|/Game/Player/BPAC_Inventory.BPAC_Inventory_C|GetInventoryMap _output_get) (Variables|/Game/Player/BPAC_Inventory.BPAC_Inventory_C|GetActiveSlotIndex _output_get))))
      (if (!= (Utilities|Array|FindItem (Variables|Default|GetSlotableItems) (.class (.Value (Utilities|Map|Find (Variables|/Game/Player/BPAC_Inventory.BPAC_Inventory_C|GetInventoryMap _output_get) (Variables|/Game/Player/BPAC_Inventory.BPAC_Inventory_C|GetActiveSlotIndex _output_get))))) -1)
        (if (Utilities|ClassIsChildOf (.class (.Value (Utilities|Map|Find (Variables|/Game/Player/BPAC_Inventory.BPAC_Inventory_C|GetInventoryMap _output_get) (Variables|/Game/Player/BPAC_Inventory.BPAC_Inventory_C|GetActiveSlotIndex _output_get)))) "/Game/Items/BP_ItemParent.BP_ItemParent_C")
          ;[1 1 1] prochazime usb sloty, zda jsou uz pouzivane
          (bind _values (Utilities|Map|Values (Variables|Default|GetItemsInSlots)))
          (for (_array_element _array_index) _values
            ;;[1 1 1] jestli je objekt ve slotu
            (if (not (Utilities|IsValid _array_element))
              (bind _returnvalue_2 (Game|SpawnActorfromClass (.class (.Value (Utilities|Map|Find (Variables|/Game/Player/BPAC_Inventory.BPAC_Inventory_C|GetInventoryMap (Variables|Default|GetInventory)) (Variables|/Game/Player/BPAC_Inventory.BPAC_Inventory_C|GetActiveSlotIndex (Variables|Default|GetInventory))))) (Math|Transform|MakeTransform (Transformation|GetSocketLocation _pcstaticmesh (Utilities|String|StringToName (Utilities|String|Append "UsbSocket" (Utilities|String|ToString(Integer) (+ _array_index 1))))) (Math|Rotator|MakeRotator (+ (.roll _returnvalue) 9e+01) (.pitch _returnvalue) (+ (.yaw _returnvalue) -9e+01)) (.transformscale (.Value (Utilities|Map|Find (Variables|/Game/Player/BPAC_Inventory.BPAC_Inventory_C|GetInventoryMap (Variables|Default|GetInventory)) (Variables|/Game/Player/BPAC_Inventory.BPAC_Inventory_C|GetActiveSlotIndex (Variables|Default|GetInventory)))))) "AlwaysSpawn" "MultiplyWithRoot" 0 0))
              (if (Utilities|IsValid _returnvalue_2)
                (bind _asbp_item_parent (Utilities|Casting|CastToBP_ItemParent _returnvalue_2)
                  (:then
                    (Utilities|Map|Add (Variables|Default|GetItemsInSlots) _array_index _asbp_item_parent)
                    (bind _returnvalue_3 (Transformation|AttachComponentToComponent _returnvalue_2 (Variables|Default|GetPcStaticMesh) (Utilities|String|StringToName (Utilities|String|Append "UsbSocket" (Utilities|String|ToString(Integer) (+ _array_index 1)))) "SnapToTarget" "SnapToTarget" "KeepWorld" true))
                    (if _returnvalue_3
                      (Physics|SetSimulatePhysics (Variables|/Game/Items/BP_ItemParent.BP_ItemParent_C|GetMainStaticMesh _asbp_item_parent) false)
                      (Default|SetAtributesfromStructtoObject (Variables|Default|GetInventory) _returnvalue_2 (.atributes (.Value (Utilities|Map|Find (Variables|/Game/Player/BPAC_Inventory.BPAC_Inventory_C|GetInventoryMap (Variables|Default|GetInventory)) (Variables|/Game/Player/BPAC_Inventory.BPAC_Inventory_C|GetActiveSlotIndex (Variables|Default|GetInventory))))) (.slotable (.Value (Utilities|Map|Find (Variables|/Game/Player/BPAC_Inventory.BPAC_Inventory_C|GetInventoryMap (Variables|Default|GetInventory)) (Variables|/Game/Player/BPAC_Inventory.BPAC_Inventory_C|GetActiveSlotIndex (Variables|Default|GetInventory))))))
                      (Default|RemoveItem (Variables|Default|GetInventory) (Variables|/Game/Player/BPAC_Inventory.BPAC_Inventory_C|GetActiveSlotIndex (Variables|Default|GetInventory)))
                      (else
                        (Development|PrintString "NEPOVEDLO SE ATTACHNUTI USBFLASHDISKU"))))
                  (:CastFailed
                    (Development|PrintString "casto to itemparent FAILED in bp_pocitac->event graph")))))))))))

(event EventBeginPlay
  (|CallParentFunction)
  (Variables|Default|SetItemsInSlots (Utilities|Map|MakeMap 0 0 1 0 2 0 3 0))
  (Utilities|Array|Add (Variables|Default|GetSlotableItems) "/Game/Items/UsbFlashDrive/BP_UsbFlashDisk.BP_UsbFlashDisk_C")
  (bind _returnvalue (Actor|GetActorOfClass "/Game/Items/Computer/BP_Computer.BP_Computer_C"))
  (Variables|Default|SetParentDevice _returnvalue))

(fn ConstructionScript)