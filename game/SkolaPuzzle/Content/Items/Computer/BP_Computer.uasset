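; BP_Computer is an interactable computer actor that shows a WBP_Computer interface on its widget component.
; On BeginPlay it creates the widget, passes itself and its APPS to it, then assigns it to the component.
; Interact hands that same widget to the first-person character's BeginOnWidegtFull, apparently for full-screen use.
; The USB add, remove and update functions are empty stubs, and an older character-owned widget path is disconnected.
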(event EventInteract
  (params (inventory :type BPAC%20Inventory%20Object%20Reference) (hitComponent :type Primitive%20Component%20Object%20Reference))
  (bind _aswbp_computer (Utilities|Casting|CastToWBP_Computer (UserInterface|GetWidget (Variables|Default|GetComputerWidget))))
  (bind _asbp_first_person_character (Utilities|Casting|CastToBP_FirstPersonCharacter (Game|GetPlayerCharacter 0)))
  (Default|BeginonWidegtFull _asbp_first_person_character _aswbp_computer))

(event EventBeginPlay
  (bind _returnvalue (UserInterface|CreateWidget "/Game/UI/Computer/WBP_Computer.WBP_Computer_C"))
  (Variables|/Game/UI/Computer/WBP_Computer.WBP_Computer_C|SetcomputerActor _returnvalue self)
  (Default|BeginEvent _returnvalue (Variables|Default|GetAPPS))
  (UserInterface|SetWidget (Variables|Default|GetComputerWidget) _returnvalue))

(fn ConstructionScript)

(fn AddUsb
  (params (usb :type BP%20Usb%20Flash%20Disk%20Object%20Reference)))

(fn RemoveUsb
  (params (usb :type BP%20Usb%20Flash%20Disk%20Object%20Reference)))

(fn UpadteUsbWidget)