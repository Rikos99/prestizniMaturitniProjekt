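; BP_Cable is a yellow network cable item that switches between a rolled and an unrolled visual state.
; On BeginPlay it starts rolled and marks itself as slotable.
; VisualRoll shows the rolled component hierarchy and enables physics on the cable mesh, while VisualUnroll shows the unrolled hierarchy and disables physics.
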(event EventBeginPlay
  (CallFunction|VisualRoll)
  (Variables|Default|SetSlotable true))

(fn ConstructionScript)

(fn VisualRoll
  (Physics|SetSimulatePhysics (Variables|Default|GetsitovyKabel-zluty) true)
  (Rendering|SetVisibility (Variables|Default|GetunrolledSceneComponent) false true)
  (Rendering|SetVisibility (Variables|Default|GetrolledSceneComponent) true true))

(fn VisualUnroll
  (Physics|SetSimulatePhysics (Variables|Default|GetsitovyKabel-zluty) false)
  (Rendering|SetVisibility (Variables|Default|GetunrolledSceneComponent) true true)
  (Rendering|SetVisibility (Variables|Default|GetrolledSceneComponent) false true))