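; BP_splineMeshTest is a test Blueprint in the Lasery items folder that builds a chain of spline meshes along a spline.
; Its construction script loops from 1 through the point count, adding an X-forward spline mesh component with a Vive pre-controller mesh between successive input keys.
; Segments use local-space positions without computed tangents, and the loop starts at key 1, skipping the segment from key 0.
; It has no runtime logic.
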(event EventBeginPlay)

(fn ConstructionScript
  (bind _spline (Variables|Default|GetSpline))
  ;[1 1 1] Comment
  (for _index (range 1 (Spline|GetNumberOfSplinePoints (Variables|Default|GetSpline)))
    (bind _returnvalue (AddComponent|AddSplineMeshComponent false))
    (SplineMesh|SetForwardAxis _returnvalue "X" true)
    (SplineMesh|SetStartandEnd _returnvalue (Class|SplineComponent|GetLocationatSplineInputKey _spline (Math|Conversions|ToFloat(Integer) _index) "Local") "0, 0, 0" (Class|SplineComponent|GetLocationatSplineInputKey _spline (Math|Conversions|ToFloat(Integer) (+ _index 1)) "Local") "0, 0, 0" true :!class /Script/Engine.SplineMeshComponent)
    (Components|StaticMesh|SetStaticMesh _returnvalue "/Engine/VREditor/Devices/Vive/VivePreControllerMesh.VivePreControllerMesh")))