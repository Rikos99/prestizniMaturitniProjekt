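; Laser emitter actor that fires a beam reflecting off actors implementing BPI_LaserBounce, with an ID label and transmitter material tinted to the laser color.
; Every tick it line-traces forward, recursively reflects on bounceable hits and rebuilds a linear spline from the hit points.
; When the last spline point moves, it destroys and recreates the spline mesh segments, which generate overlap events, to show the beam.
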(event EventBeginPlay
  (bind _spline (Variables|Default|GetSpline))
  (Utilities|FlowControl|Sequence
    (:then_0
      (Variables|Default|SetLastPoint (.position (Spline|GetSplinePointAt _spline (- (Spline|GetNumberOfSplinePoints _spline) 1) "Local"))))))

(event EventTick
  (params (DeltaSeconds :type Float%20%28single-precision%29))
  (bind _spline (Variables|Default|GetSpline))
  (bind _spline_2 (Variables|Default|GetSpline))
  (CallFunction|CheckBounce)
  (if (Utilities|Operators|NotEqual(!=) (.position (Spline|GetSplinePointAt _spline (- (Spline|GetNumberOfSplinePoints _spline) 1) "Local")) (Variables|Default|GetLastPoint) 0.0)
    (CallFunction|UpdateSplineMesh)
    (Variables|Default|SetLastPoint (.position (Spline|GetSplinePointAt _spline_2 (- (Spline|GetNumberOfSplinePoints _spline_2) 1) "Local")))))

(fn ConstructionScript
  (bind _idtext (Variables|Default|GetidText))
  (Rendering|Components|TextRender|SetText _idtext (Utilities|Text|ToText(Name) (Variables|Default|GetlaserId)))
  (Rendering|Components|TextRender|SetTextRenderColor _idtext (Variables|Default|GetLaserColor))
  (bind _returnvalue (Rendering|Material|CreateDynamicMaterialInstance (Variables|Default|Gettransmitter) 0 "/Game/Materials/lasery/M_transmitter.M_transmitter" "None" :!class /Script/Engine.PrimitiveComponent))
  (Rendering|Material|SetVectorParameterValue _returnvalue "LaserColor" (Math|Conversions|ToLinearColor(Color) (Variables|Default|GetLaserColor)) :!class /Script/Engine.MaterialInstanceDynamic)
  (bind _output_get (Variables|Default|SetMaterial _returnvalue))
  (Rendering|Material|SetMaterial (Variables|Default|Gettransmitter) 0 _output_get))

(fn CheckBounce
  (Variables|Default|SetSplineInputKey 0.0)
  (bind _output_get (Variables|Default|SetCurrentLocation (Transformation|GetWorldLocation (Variables|Default|GetArrow))))
  (Variables|Default|SetDirection (Transformation|GetActorForwardVector self))
  (Spline|ClearSplinePoints (Variables|Default|GetSpline) false)
  (Class|SplineComponent|AddPoint (Variables|Default|GetSpline) (Utilities|Struct|MakeSplinePoint (Variables|Default|GetSplineInputKey) (Math|Transform|InverseTransformLocation (Transformation|GetWorldTransform (Variables|Default|GetSpline)) _output_get) "0.000000,0.000000,0.000000" "0.000000,0.000000,0.000000" "0.000000,0.000000,0.000000" "1.000000,1.000000,1.000000" "Linear") false)
  (Math|Float|IncrementFloat (Variables|Default|GetSplineInputKey)
    (:%20%20
      (bind (_outhit _returnvalue) (Collision|LineTraceByChannel (Variables|Default|GetCurrentLocation) (+ (Variables|Default|GetCurrentLocation) (* (Variables|Default|GetDirection) (Variables|Default|GetTraceLength))) "TraceTypeQuery1" false 0 (Variables|Default|GetDraw%20Debug%20Type) true "(R=1.000000,G=0.000000,B=0.000000,A=1.000000)" "(R=0.000000,G=1.000000,B=0.000000,A=1.000000)" 1.0))
      (if _returnvalue
        (CallFunction|NewBounce (.location _outhit) (.normal _outhit) (.hitactor _outhit) (.hitcomponent _outhit))
        (else
          (return))))))

(fn NewBounce
  (params (hitLocation :type Vector) (hitNormal :type Vector) (hitActor :type Actor%20Object%20Reference) (hitComponent :type Primitive%20Component%20Object%20Reference))
  (Variables|Default|SetDirection (- (Math|Vector|Normalize (- (Variables|Default|GetCurrentLocation) hitLocation)) (* hitNormal (* (Math|Vector|DotProduct (Math|Vector|Normalize (- (Variables|Default|GetCurrentLocation) hitLocation)) hitNormal) 2.0))))
  (bind _output_get (Variables|Default|SetCurrentLocation hitLocation))
  (Rendering|Debug|DrawDebugSphere _output_get 5.0 12 "(R=0.769821,G=0.000000,B=1.000000,A=1.000000)" 0.0)
  ;[1 1 1] vytvoreni a pridani noveho spline bodu
  (Class|SplineComponent|AddPoint (Variables|Default|GetSpline) (Utilities|Struct|MakeSplinePoint (Variables|Default|GetSplineInputKey) (Math|Transform|InverseTransformLocation (Transformation|GetWorldTransform (Variables|Default|GetSpline)) _output_get) "0.000000,0.000000,0.000000" "0.000000,0.000000,0.000000" "0.000000,0.000000,0.000000" "1.000000,1.000000,1.000000" "Linear") true)
  ;[1 1 1] inkrementace indexu bodu spline
  (Math|Float|IncrementFloat (Variables|Default|GetSplineInputKey)
    (:%20%20
      ;[1 1 1] jestli line trace trefil obejekt, od ktereho se laser muze odrazit
      (if (Utilities|DoesObjectImplementInterface hitActor "/Game/Items/Lasery/BPI_LaserBounce.BPI_LaserBounce_C")
        (bind (_outhit _returnvalue) (Collision|LineTraceByChannel (Variables|Default|GetCurrentLocation) (- (Variables|Default|GetCurrentLocation) (* (Variables|Default|GetDirection) (Variables|Default|GetTraceLength))) "TraceTypeQuery1" false (Utilities|Array|MakeArray hitActor) (Variables|Default|GetDraw%20Debug%20Type) false "(R=1.000000,G=0.000000,B=0.033409,A=1.000000)" "(R=1.000000,G=0.602256,B=0.000000,A=1.000000)" 1.0))
        (if _returnvalue
          (CallFunction|NewBounce (.location _outhit) (.normal _outhit) (.hitactor _outhit) (.hitcomponent _outhit))
          (else
            (return)))
        (else
          ;[1 1 1] updatnuti splinu, aby se nove body na splinu ukazaly
          (Spline|UpdateSpline (Variables|Default|GetSpline))
          (return))))))

(fn UpdateSplineMesh
  ;[1 1 1] Comment
  (CallFunction|RemoveOldSplineMeshes)
  (for _index (range 0 (- (Spline|GetNumberOfSplinePoints (Variables|Default|GetSpline)) 1))
    (bind _returnvalue (AddComponent|AddSplineMeshComponent false))
    (Utilities|Array|Add (Variables|Default|GetSplineMeshes) _returnvalue)
    (Utilities|FlowControl|Sequence
      (:then_0
        (Collision|SetCollisionEnabled _returnvalue "QueryOnly")
        (Collision|SetCollisionProfileName _returnvalue "OverlapAllDynamic" true :!class /Script/Engine.PrimitiveComponent)
        (Variables|/Script/Engine.PrimitiveComponent|SetbGenerateOverlapEvents _returnvalue true)
        (SplineMesh|SetForwardAxis _returnvalue (Variables|Default|GetIn%20Forward%20Axis) false))
      (:then_1
        (SplineMesh|SetStartandEnd _returnvalue (+ (Spline|GetLocationatSplinePoint (Variables|Default|GetSpline) _index "Local") (Variables|Default|GetLaserFromActorOriginOffset)) "0, 0, 0" (+ (Spline|GetLocationatSplinePoint (Variables|Default|GetSpline) (+ _index 1) "Local") (Variables|Default|GetLaserFromActorOriginOffset)) "0, 0, 0" true :!class /Script/Engine.SplineMeshComponent)
        (Transformation|SetMobility _returnvalue "Movable")
        (Components|StaticMesh|SetStaticMesh _returnvalue (Variables|Default|GetLaserMesh))
        (Development|PrintString (Utilities|String|ToString(Vector) (Transformation|GetWorldScale _returnvalue)))))))

(fn RemoveOldSplineMeshes
  (bind _splinemeshes (Variables|Default|GetSplineMeshes))
  (for _array_element _splinemeshes
    (Components|DestroyComponent _array_element))
  (Utilities|Array|Clear _splinemeshes))