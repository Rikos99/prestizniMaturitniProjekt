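; Test actor, judging by its name, that builds box-shaped procedural geometry along a spline in its Construction Script.
; Each point adds eight corners from the direction to the next point, Width and Height, centered on that point rather than mid-segment.
; Corner and triangle arrays accumulate while the mesh section is recreated each pass, but the hardcoded indices only address the first box.
; An alternative SplineMeshComponent loop is left unconnected.
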(event EventBeginPlay)

(fn ConstructionScript
  (bind _spline (Variables|Default|GetSpline))
  (for _index (range 0 (Spline|GetNumberOfSplinePoints (Variables|Default|GetSpline)))
    (Utilities|FlowControl|Sequence
      (:then_0
        (LocalVariables|Setv2 (Spline|GetLocationatSplinePoint _spline (+ _index 1) "Local"))
        (LocalVariables|Setv1 (Spline|GetLocationatSplinePoint _spline _index "Local"))
        (LocalVariables|Setdirection (Math|Vector|Normalize (- (Spline|GetLocationatSplinePoint _spline (+ _index 1) "Local") (Spline|GetLocationatSplinePoint _spline _index "Local"))))
        (LocalVariables|SethalfLength (/ (Math|Vector|VectorLength (- (Spline|GetLocationatSplinePoint _spline (+ _index 1) "Local") (Spline|GetLocationatSplinePoint _spline _index "Local"))) 2.0))
        (LocalVariables|Setright (Math|Vector|Normalize (Math|Vector|CrossProduct (LocalVariables|Getdirection) (Math|Vector|VectorUp))))
        (LocalVariables|Setup (Math|Vector|Normalize (Math|Vector|CrossProduct (LocalVariables|Getdirection) (LocalVariables|Getright))))
        (LocalVariables|SethalfLengthOffset (* (LocalVariables|Getdirection) (LocalVariables|GethalfLength)))
        (LocalVariables|SethalfWidthOffset (* (LocalVariables|Getright) (/ (LocalVariables|Getwidth) 2.0)))
        (LocalVariables|SethalfHeightOffset (* (LocalVariables|Getup) (/ (LocalVariables|Getheight) 2.0)))
        (Utilities|FlowControl|Sequence
          (:then_0
            (Utilities|Array|Add (LocalVariables|GetCorners) (Utilities|Operators|Subtract (LocalVariables|Getv1) (LocalVariables|GethalfWidthOffset) (LocalVariables|GethalfHeightOffset) (LocalVariables|GethalfLengthOffset))))
          (:then_1
            (Utilities|Array|Add (LocalVariables|GetCorners) (Utilities|Operators|Subtract (+ (LocalVariables|Getv1) (LocalVariables|GethalfWidthOffset)) (LocalVariables|GethalfHeightOffset) (LocalVariables|GethalfLengthOffset))))
          (:then_2
            (Utilities|Array|Add (LocalVariables|GetCorners) (- (+ (LocalVariables|Getv1) (LocalVariables|GethalfWidthOffset) (LocalVariables|GethalfHeightOffset)) (LocalVariables|GethalfLengthOffset))))
          (:then_3
            (Utilities|Array|Add (LocalVariables|GetCorners) (- (+ (- (LocalVariables|Getv1) (LocalVariables|GethalfWidthOffset)) (LocalVariables|GethalfHeightOffset)) (LocalVariables|GethalfLengthOffset))))
          (:then_4
            (Utilities|FlowControl|Sequence
              (:then_0
                (Utilities|Array|Add (LocalVariables|GetCorners) (+ (Utilities|Operators|Subtract (LocalVariables|Getv1) (LocalVariables|GethalfWidthOffset) (LocalVariables|GethalfHeightOffset)) (LocalVariables|GethalfLengthOffset))))
              (:then_1
                (Utilities|Array|Add (LocalVariables|GetCorners) (+ (- (+ (LocalVariables|Getv1) (LocalVariables|GethalfWidthOffset)) (LocalVariables|GethalfHeightOffset)) (LocalVariables|GethalfLengthOffset))))
              (:then_2
                (Utilities|Array|Add (LocalVariables|GetCorners) (+ (LocalVariables|Getv1) (LocalVariables|GethalfWidthOffset) (LocalVariables|GethalfHeightOffset) (LocalVariables|GethalfLengthOffset))))
              (:then_3
                (Utilities|Array|Add (LocalVariables|GetCorners) (+ (- (LocalVariables|Getv1) (LocalVariables|GethalfWidthOffset)) (LocalVariables|GethalfHeightOffset) (LocalVariables|GethalfLengthOffset))))))))
      (:then_1
        (for _array_element (Utilities|String|ParseIntoArray "0, 1, 2, 0, 2, 3, 4, 5, 6, 4, 6, 7, 0, 4, 7, 0, 7, 3, 1, 5, 6, 1, 6, 2, 3, 2, 6, 3, 6, 7, 0, 1, 5, 0, 5, 4" ",")
          (Utilities|Array|Add (LocalVariables|Gettriangles) (Math|Conversions|ToInteger(Byte) _array_element)))
        (Class|ProceduralMeshComponent|CreateMeshSectionLinearColor (Variables|Default|GetProceduralMesh) 0 (LocalVariables|GetCorners) (LocalVariables|Gettriangles) (Utilities|Array|MakeArray "0.000000,0.000000,-1.000000" "0.000000,0.000000,1.000000" "-1.000000,0.000000,0.000000" "1.000000,0.000000,0.000000" "0.000000,-1.000000,0.000000" "0.000000,1.000000,0.000000") (Utilities|Array|MakeArray "" "(X=1.000000,Y=0.000000)" "(X=1.000000,Y=1.000000)" "(X=0.000000,Y=1.000000)") 0 0 0 0 0 false false)))))