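; BP_LaserMirror is an interactable mirror actor that the player can rotate, apparently for a laser mechanic.
; Interact puts BP_FirstPersonCharacter into focused interaction, registers the mirror as its hand interaction item, and disables camera and character movement.
; PlayerMouse turns horizontal mouse input, scaled by RotationSpeed, into local yaw; vertical input is unused.
; The graph contains no beam reflection or focus-exit logic.
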(event Custom|PlayerMouse
  (params (x :type Float%20%28double-precision%29) (y :type Float%20%28double-precision%29))
  ;[1 1 1] jestli ze otacim kolecko
  (Transformation|AddActorLocalRotation (Math|Rotator|MakeRotator 0.0 0.0 (* x (Variables|Default|GetrotationSpeed))) false false))

(event EventBeginPlay)

(event Collision|EventActorBeginOverlap
  (params (OtherActor :type Actor%20Object%20Reference)))

(event EventTick
  (params (DeltaSeconds :type Float%20%28single-precision%29)))

(event EventInteract
  (params (inventory :type BPAC%20Inventory%20Object%20Reference) (hitComponent :type Primitive%20Component%20Object%20Reference))
  (bind _asbp_first_person_character (Utilities|Casting|CastToBP_FirstPersonCharacter (Game|GetPlayerCharacter 0)))
  (Variables|/Game/Player/BP_FirstPersonCharacter.BP_FirstPersonCharacter_C|SetFocusedInteract _asbp_first_person_character true)
  (Variables|/Game/Player/BP_FirstPersonCharacter.BP_FirstPersonCharacter_C|SetHandInteractionItem _asbp_first_person_character self)
  (Variables|/Game/Player/BP_FirstPersonCharacter.BP_FirstPersonCharacter_C|SetMoveCamera _asbp_first_person_character false)
  (Pawn|Components|CharacterMovement|SetMovementMode (Variables|/Script/Engine.Character|GetCharacterMovement _asbp_first_person_character) "MOVE_None" 0))

(fn ConstructionScript)