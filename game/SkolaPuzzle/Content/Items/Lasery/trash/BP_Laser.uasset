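; BP_Laser is a laser beam actor that uses a Cylinder component as the beam between two points.
; OnSpawn scales the cylinder's cross-section by Width and its length by the Start-to-End distance, then shifts it half that distance along local X.
; It does not set actor position or rotation.
; It also prints the actor's name and draws long-lived debug spheres at both endpoints.
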(fn ConstructionScript)

(fn OnSpawn
  (params (start :type Vector) (end :type Vector))
  (bind _returnvalue (- start end))
  (bind _width (Variables|Default|Getwidth))
  (bind _returnvalue_2 (Math|Vector|VectorLength _returnvalue))
  (bind _returnvalue_3 (/ _width 1e+02))
  (Development|PrintString (Utilities|GetDisplayName self) true true "(R=1.000000,G=0.000000,B=0.307249,A=1.000000)" 6e+01)
  (Rendering|Debug|DrawDebugSphere start 5e+01 12 "(R=0.000000,G=0.260342,B=1.000000,A=1.000000)" 4e+01)
  (Rendering|Debug|DrawDebugSphere end 49.0 12 "(R=1.000000,G=0.000000,B=0.070807,A=1.000000)" 4e+01)
  (Utilities|FlowControl|Sequence
    (:then_0
      (Transformation|SetRelativeScale3D (Variables|Default|GetCylinder) (Math|Vector|MakeVector _returnvalue_3 _returnvalue_3 (/ _returnvalue_2 1e+02))))
    (:then_1
      (Transformation|SetRelativeLocation (Variables|Default|GetCylinder) (Math|Vector|MakeVector (/ _returnvalue_2 2.0) 0.0 0.0) false false))))