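; Laser generator actor that every tick traces a beam from its arrow along its forward vector and reflects it off actors implementing BPI_LaserBounce.
; Recursive NewBounce calls record each hit as a linear spline point.
; A non-bouncing hit ends the chain, destroying old BP_Laser actors and spawning new ones between points; a missed trace skips this rebuild.
; The spline-mesh and BPI_HitByLaser paths are never called.
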(event EventTick
  (params (DeltaSeconds :type Float%20%28single-precision%29))
  (CallFunction|CheckBounce))

(fn ConstructionScript)

(fn CheckBounce
  (Variables|Default|SetSplineInputKey 0.0)
  (bind _output_get (Variables|Default|SetCurrentLocation (Transformation|GetWorldLocation (Variables|Default|GetArrow))))
  (Variables|Default|SetDirection (Transformation|GetActorForwardVector self))
  (Spline|ClearSplinePoints (Variables|Default|GetSpline) false)
  (Class|SplineComponent|AddPoint (Variables|Default|GetSpline) (Utilities|Struct|MakeSplinePoint (Variables|Default|GetSplineInputKey) (Math|Transform|InverseTransformLocation (Transformation|GetWorldTransform (Variables|Default|GetSpline)) _output_get) "0.000000,0.000000,0.000000" "0.000000,0.000000,0.000000" "0.000000,0.000000,0.000000" "1.000000,1.000000,1.000000" "Linear") false)
  (Math|Float|IncrementFloat (Variables|Default|GetSplineInputKey)
    (:%20%20
      (bind (_outhit _returnvalue) (Collision|LineTraceByChannel (Variables|Default|GetCurrentLocation) (+ (Variables|Default|GetCurrentLocation) (* (Variables|Default|GetDirection) (Variables|Default|GetTraceLength))) "TraceTypeQuery1" false (Variables|Default|GetLasers) "ForOneFrame" true "(R=1.000000,G=0.000000,B=0.000000,A=1.000000)" "(R=0.000000,G=1.000000,B=0.000000,A=1.000000)" 1.0))
      (if _returnvalue
        (CallFunction|NewBounce (.location _outhit) (.normal _outhit) (.hitactor _outhit) (.hitcomponent _outhit))
        (else
          (return))))))

(fn NewBounce
  (params (hitLocation :type Vector) (hitNormal :type Vector) (hitActor :type Actor%20Object%20Reference) (hitComponent :type Primitive%20Component%20Object%20Reference))
  (bind _array (Utilities|Array|MakeArray hitActor 0))
  (Variables|Default|SetDirection (- (Math|Vector|Normalize (- (Variables|Default|GetCurrentLocation) hitLocation)) (* hitNormal (* (Math|Vector|DotProduct (Math|Vector|Normalize (- (Variables|Default|GetCurrentLocation) hitLocation)) hitNormal) 2.0))))
  (bind _output_get (Variables|Default|SetCurrentLocation hitLocation))
  (Rendering|Debug|DrawDebugSphere _output_get 5.0 12 "(R=0.769821,G=0.000000,B=1.000000,A=1.000000)" 0.0)
  ;[1 1 1] vytvoreni a pridani noveho spline bodu
  (Class|SplineComponent|AddPoint (Variables|Default|GetSpline) (Utilities|Struct|MakeSplinePoint (Variables|Default|GetSplineInputKey) (Math|Transform|InverseTransformLocation (Transformation|GetWorldTransform (Variables|Default|GetSpline)) _output_get) "0.000000,0.000000,0.000000" "0.000000,0.000000,0.000000" "0.000000,0.000000,0.000000" "1.000000,1.000000,1.000000" "Linear") false)
  ;[1 1 1] inkrementace indexu bodu spline
  (Math|Float|IncrementFloat (Variables|Default|GetSplineInputKey)
    (:%20%20
      ;[1 1 1] jestli line trace trefil obejekt, od ktereho se laser muze odrazit
      (if (Utilities|DoesObjectImplementInterface hitActor "/Game/Items/Lasery/BPI_LaserBounce.BPI_LaserBounce_C")
        (Utilities|Array|AppendArray _array (Variables|Default|GetLasers))
        (bind (_outhit _returnvalue) (Collision|LineTraceByChannel (Variables|Default|GetCurrentLocation) (- (Variables|Default|GetCurrentLocation) (* (Variables|Default|GetDirection) (Variables|Default|GetTraceLength))) "TraceTypeQuery1" false _array "ForOneFrame" false "(R=1.000000,G=0.000000,B=0.033409,A=1.000000)" "(R=1.000000,G=0.602256,B=0.000000,A=1.000000)" 1.0))
        (if _returnvalue
          (CallFunction|NewBounce (.location _outhit) (.normal _outhit) (.hitactor _outhit) (.hitcomponent _outhit))
          (else
            (return)))
        (elif true
          ;[1 1 1] updatnuti splinu, aby se nove body na splinu ukazaly
          (Spline|UpdateSpline (Variables|Default|GetSpline))
          (CallFunction|RemoveOldLaser)
          (CallFunction|MakeLaser)
          (return))))))

(fn MakeLaser
  (bind _spline (Variables|Default|GetSpline))
  (for _index (range 0 (- (Spline|GetNumberOfSplinePoints (Variables|Default|GetSpline)) 0))
    (bind _returnvalue (Game|SpawnActorfromClass "/Game/Items/Lasery/trash/BP_Laser.BP_Laser_C" (Math|Transform|MakeTransform (Spline|GetLocationatSplinePoint _spline _index "World") (Math|Rotator|FindLookatRotation (Spline|GetLocationatSplinePoint _spline _index "World") (Spline|GetLocationatSplinePoint _spline (+ _index 1) "World")) "1.000000,1.000000,1.000000") "Undefined" "MultiplyWithRoot" 0 0))
    (Default|OnSpawn _returnvalue (Spline|GetLocationatSplinePoint _spline _index "World") (Spline|GetLocationatSplinePoint _spline (+ _index 1) "World"))
    (Utilities|Array|Add (Variables|Default|GetLasers) _returnvalue)))

(fn UpdateSplineMesh
  (bind _lasermesh (Variables|Default|GetLaserMesh))
  (bind _spline (Variables|Default|GetSpline))
  (bind _spline_2 (Variables|Default|GetSpline))
  (bind _returnvalue (StaticMesh|GetBoundingBox _lasermesh))
  (Variables|Default|SetXLenght (.x (+ (Math|Vector|VectorGetAbs (.min _returnvalue)) (Math|Vector|VectorGetAbs (.max _returnvalue)))))
  (for _index (range 0 (Math|Float|Truncate (/ (Spline|GetSplineLength (Variables|Default|GetSpline)) (Variables|Default|GetXLenght))))
    (bind _returnvalue_2 (AddComponent|AddSplineMeshComponent false))
    (Collision|SetCollisionEnabled _returnvalue_2 "QueryOnly")
    (SplineMesh|SetForwardAxis _returnvalue_2 "X" true)
    (Components|StaticMesh|SetStaticMesh _returnvalue_2 (Variables|Default|GetLaserMesh))
    (Transformation|SetMobility _returnvalue_2 "Movable")
    (SplineMesh|SetStartandEnd _returnvalue_2 (Spline|GetLocationatDistanceAlongSpline _spline_2 (* _index (Variables|Default|GetXLenght)) "Local") (Math|Vector|ClampVectorSize (Spline|GetTangentatDistanceAlongSpline _spline_2 (* _index (Variables|Default|GetXLenght)) "Local") 0.0 (Variables|Default|GetXLenght)) (Spline|GetLocationatDistanceAlongSpline _spline (* (+ _index 1) (Variables|Default|GetXLenght)) "Local") (Math|Vector|ClampVectorSize (Spline|GetTangentatDistanceAlongSpline _spline (* (+ _index 1) (Variables|Default|GetXLenght)) "Local") 0.0 (Variables|Default|GetXLenght)) true :!class /Script/Engine.SplineMeshComponent)
    (Development|PrintString (Utilities|String|ToString(Vector) (Spline|GetLocationatDistanceAlongSpline _spline_2 (* _index (Variables|Default|GetXLenght)) "Local")))))

(fn RemoveOldLaser
  (bind _lasers (Variables|Default|GetLasers))
  (for _array_element _lasers
    (Actor|DestroyActor _array_element))
  (Utilities|Array|Clear _lasers))