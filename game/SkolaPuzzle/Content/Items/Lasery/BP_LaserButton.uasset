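; BP_LaserButton is a laser button actor whose reactions are so far only debug prints.
; On BeginPlay it binds begin and end overlap events on its LaserButtonHitBox component.
; Each overlap prints the names of the other actor and component in red.
; A custom OnGetHitbyLaser event prints a greeting, with no button state or activation logic.
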(event Custom|BeginOverlap
  (params (OverlappedComponent :type Primitive%20Component%20Object%20Reference) (OtherActor :type Actor%20Object%20Reference) (OtherComp :type Primitive%20Component%20Object%20Reference) (OtherBodyIndex :type Integer) (bFromSweep :type Boolean) (SweepResult :type Hit%20Result%20Structure%20%28by%20ref%29))
  (Development|PrintString (Utilities|String|Append (Utilities|GetDisplayName OtherActor) (Utilities|GetDisplayName OtherComp) "\\") true true "(R=1.000000,G=0.000000,B=0.086574,A=1.000000)"))

(event Custom|EndOverlap
  (params (OverlappedComponent :type Primitive%20Component%20Object%20Reference) (OtherActor :type Actor%20Object%20Reference) (OtherComp :type Primitive%20Component%20Object%20Reference) (OtherBodyIndex :type Integer))
  (Development|PrintString (Utilities|String|Append (Utilities|GetDisplayName OtherActor) (Utilities|GetDisplayName OtherComp) "\\") true true "(R=1.000000,G=0.000000,B=0.029677,A=1.000000)"))

(event EventBeginPlay
  (bind _laserbuttonhitbox (Variables|Default|GetlaserButtonHitBox))
  (Collision|BindEventtoOnComponentBeginOverlap _laserbuttonhitbox (delegate Custom|BeginOverlap))
  (Collision|BindEventtoOnComponentEndOverlap _laserbuttonhitbox (delegate Custom|EndOverlap))
  (Development|PrintString "BEGGIIIIN"))

(event Collision|EventActorBeginOverlap
  (params (OtherActor :type Actor%20Object%20Reference)))

(event EventTick
  (params (DeltaSeconds :type Float%20%28single-precision%29)))

(event EventOnGetHitbyLaser
  (Development|PrintString "Hello"))

(fn ConstructionScript)