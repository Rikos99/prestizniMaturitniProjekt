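; Laser generator actor that fires a beam from its arrow and bounces it off actors implementing BPI_LaserBounce.
; Every tick it line-traces forward and recursively traces reflection vectors, recording hit points and ignoring actors of configured classes.
; When the path ends on a non-bouncing hit and differs from last tick's, it respawns BP_Laser segments between points.
; A missed trace leaves existing segments untouched.
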(event EventTick
  (params (DeltaSeconds :type Float%20%28single-precision%29))
  (CallFunction|CheckBounce))

(fn ConstructionScript)

(fn CheckBounce
  (bind _lasersends (Variables|Default|GetLasersEnds))
  (Variables|Default|SetpreviousLasersEnds _lasersends)
  (Utilities|Array|Clear _lasersends)
  (Variables|Default|SetCurrentLocation (Transformation|GetWorldLocation (Variables|Default|GetArrow)))
  (Variables|Default|SetDirection (Transformation|GetActorForwardVector self))
  (Utilities|Array|Add (Variables|Default|GetLasersEnds) (Variables|Default|GetCurrentLocation))
  (bind _actors (CallFunction|GetIgnoreActors))
  (bind (_outhit _returnvalue) (Collision|LineTraceByChannel (Variables|Default|GetCurrentLocation) (+ (Variables|Default|GetCurrentLocation) (* (Variables|Default|GetDirection) (Variables|Default|GetTraceLength))) "TraceTypeQuery1" false _actors "ForOneFrame" true "(R=1.000000,G=0.000000,B=0.000000,A=1.000000)" "(R=0.000000,G=1.000000,B=0.000000,A=1.000000)" 1.0))
  (if _returnvalue
    (Utilities|Array|Add (Variables|Default|GetLasersEnds) (.location _outhit))
    (CallFunction|NewBounce (.location _outhit) (.normal _outhit) (.hitactor _outhit) (.hitcomponent _outhit))
    (else
      (return))))

(fn NewBounce
  (params (hitLocation :type Vector) (hitNormal :type Vector) (hitActor :type Actor%20Object%20Reference) (hitComponent :type Primitive%20Component%20Object%20Reference))
  (Variables|Default|SetDirection (- (Math|Vector|Normalize (- (Variables|Default|GetCurrentLocation) hitLocation)) (* hitNormal (* (Math|Vector|DotProduct (Math|Vector|Normalize (- (Variables|Default|GetCurrentLocation) hitLocation)) hitNormal) 2.0))))
  (bind _output_get (Variables|Default|SetCurrentLocation hitLocation))
  (Rendering|Debug|DrawDebugSphere _output_get 5.0 12 "(R=0.769821,G=0.000000,B=1.000000,A=1.000000)" 0.0)
  ;[1 1 1] jestli line trace trefil obejekt, od ktereho se laser muze odrazit
  (if (Utilities|DoesObjectImplementInterface hitActor "/Game/Items/Lasery/BPI_LaserBounce.BPI_LaserBounce_C")
    (bind _actors (CallFunction|GetIgnoreActors))
    (bind (_outhit _returnvalue) (Collision|LineTraceByChannel (Variables|Default|GetCurrentLocation) (- (Variables|Default|GetCurrentLocation) (* (Variables|Default|GetDirection) (Variables|Default|GetTraceLength))) "TraceTypeQuery1" false _actors "ForOneFrame" false "(R=1.000000,G=0.000000,B=0.033409,A=1.000000)" "(R=1.000000,G=0.602256,B=0.000000,A=1.000000)" 1.0))
    (if _returnvalue
      (Utilities|Array|Add (Variables|Default|GetLasersEnds) (.location _outhit))
      (CallFunction|NewBounce (.location _outhit) (.normal _outhit) (.hitactor _outhit) (.hitcomponent _outhit))
      (else
        (return)))
    (elif (not (Utilities|Array|Identical (Variables|Default|GetLasersEnds) (Variables|Default|GetpreviousLasersEnds)))
      (CallFunction|RemoveOldLaser)
      (CallFunction|MakeLaser)
      (Development|PrintString "update LSER" true true "(R=1.000000,G=0.000000,B=0.810442,A=1.000000)")
      (return))))

(fn MakeLaser
  (bind _lasersends (Variables|Default|GetLasersEnds))
  (Utilities|FlowControl|Sequence
    (:then_0
      (for _index (range 0 (- (Utilities|Array|Length _lasersends) 2))
        (bind _returnvalue (Game|SpawnActorfromClass "/Game/Items/Lasery/BP_Laser.BP_Laser_C" (Math|Transform|MakeTransform (Utilities|Array|Get(acopy) _lasersends _index) (Math|Rotator|FindLookatRotation (Utilities|Array|Get(acopy) _lasersends _index) (Utilities|Array|Get(acopy) _lasersends (+ _index 1))) "1.000000,1.000000,1.000000") "Undefined" "MultiplyWithRoot" 0 0))
        (Default|OnSpawn _returnvalue (Utilities|Array|Get(acopy) _lasersends _index) (Utilities|Array|Get(acopy) _lasersends (+ _index 1)))
        (Utilities|Array|Add (Variables|Default|GetLasers) _returnvalue)))
    (:then_1
      (for (_array_element _array_index) _lasersends
        (Development|PrintString (Utilities|String|Append (Utilities|String|ToString(Integer) _array_index) " " (Utilities|String|ToString(Vector) _array_element)) true true "(R=0.313520,G=1.000000,B=0.000000,A=1.000000)" 8e+01)))))

(fn RemoveOldLaser
  (bind _lasers (Variables|Default|GetLasers))
  (for _array_element _lasers
    (Actor|DestroyActor _array_element))
  (Utilities|Array|Clear _lasers)
  (Development|PrintString "old lasers removed"))

(fn RefireLineTrace
  (params (start :type Vector) (end :type Vector)))

(fn GetIgnoreActors
  (Utilities|Array|Clear (LocalVariables|GetNewLocalVar))
  (for _array_element (Variables|Default|GetactorsToIgnore)
    (bind _outactors (Actor|GetAllActorsOfClass _array_element))
    (Utilities|Array|AppendArray (LocalVariables|GetNewLocalVar) _outactors))
  (return (LocalVariables|GetNewLocalVar)))