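; Laser receiver that finishes its task through BPACTaskActor once an allowed laser has been held on it for about three seconds.
; A looping timer box-checks at the Arrow for BP_LaserGenerator actors with allowed LaserIds and draws a debug box.
; A match starts a counter timer, losing it resets the count, and OnFinished fires on every check past the threshold.
; The construction script shows the allowed IDs on a TextRender.
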(event Custom|BeginOverlap
  (params (OverlappedComponent :type Primitive%20Component%20Object%20Reference) (OtherActor :type Actor%20Object%20Reference) (OtherComp :type Primitive%20Component%20Object%20Reference) (OtherBodyIndex :type Integer) (bFromSweep :type Boolean) (SweepResult :type Hit%20Result%20Structure%20%28by%20ref%29))
  ;[1 1 1] Comment
  (Development|PrintString (Utilities|String|Append (Utilities|GetDisplayName OtherActor) (Utilities|GetDisplayName OtherComp) "\\") true true "(R=1.000000,G=0.000000,B=0.086574,A=1.000000)"))

(event Custom|CustomEvent
  (bind _arrow (Variables|Default|GetArrow))
  (bind _returnvalue (Transformation|GetWorldLocation _arrow))
  (bind _outactors (Collision|BoxOverlapActors _returnvalue "4.000000,12.000000,10.000000" (Utilities|Array|MakeArray "ObjectTypeQuery1" "ObjectTypeQuery2" "ObjectTypeQuery4") "/Game/Items/Lasery/BP_LaserGenerator.BP_LaserGenerator_C" :!class /Script/Engine.KismetSystemLibrary))
  (Rendering|Debug|DrawDebugBox _returnvalue "4.000000,12.000000,10.000000" "(R=1.000000,G=0.000000,B=0.704562,A=1.000000)" (Transformation|GetActorRotation) 0.0 1.0)
  (Utilities|FlowControl|Sequence
    (:then_0
      (bind _bool (CallFunction|IsThereGoodLaser _outactors))
      (Variables|Default|SetCurValue _bool))
    (:then_1
      (if (!= (Variables|Default|GetLastValue) (Variables|Default|GetCurValue))
        (if (Variables|Default|GetCurValue)
          (bind _returnvalue_2 (Utilities|Time|SetTimerbyEvent (delegate Custom|CustomEvent_0) 0.1 true))
          (Variables|Default|SetLastValue true)
          (else
            (Utilities|Time|ClearandInvalidateTimerbyHandle _returnvalue_2)
            (Variables|Default|Setcount 0)
            (Variables|Default|SetLastValue false)))))
    (:then_2
      (if (> (Variables|Default|Getcount) 30)
        (Default|OnFinished (Variables|Default|GetBPAC_TaskActor))))))

(event Custom|EndOverlap
  (params (OverlappedComponent :type Primitive%20Component%20Object%20Reference) (OtherActor :type Actor%20Object%20Reference) (OtherComp :type Primitive%20Component%20Object%20Reference) (OtherBodyIndex :type Integer))
  ;[1 1 1] Comment
  (Development|PrintString (Utilities|String|Append (Utilities|GetDisplayName OtherActor) (Utilities|GetDisplayName OtherComp) "\\") true true "(R=1.000000,G=0.000000,B=0.029677,A=1.000000)"))

(event Custom|CustomEvent_0
  (Math|Integer|IncrementInt (Variables|Default|Getcount)))

(event EventBeginPlay
  (Utilities|Time|SetTimerbyEvent (delegate Custom|CustomEvent) 0.1 true))

(fn ConstructionScript
  (for _array_element (Variables|Default|GetLaserIdAllowed)
    (LocalVariables|Setstring (Utilities|String|Append (LocalVariables|Getstring) (Utilities|String|ToString(Name) _array_element))))
  (Rendering|Components|TextRender|SetText (Variables|Default|GetTextRender) (Utilities|Text|ToText(String) (LocalVariables|Getstring))))

(fn IsThereGoodLaser
  (params (Array :type Array%20of%20Actor%20Object%20References))
  (for _array_element Array
    (bind _asbp_laser_generator (Utilities|Casting|CastToBP_LaserGenerator _array_element))
    (if (Utilities|Array|ContainsItem (Variables|Default|GetLaserIdAllowed) (Variables|/Game/Items/Lasery/BP_LaserGenerator.BP_LaserGenerator_C|GetlaserId _asbp_laser_generator))
      (LocalVariables|SetNewLocalVar true)))
  (return (LocalVariables|GetNewLocalVar)))