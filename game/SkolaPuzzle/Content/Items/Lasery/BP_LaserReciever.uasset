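; Laser receiver puzzle actor that switches connected actors on or off according to the laser IDs it accepts.
; Each Tick, a debug-drawn box overlap above its arrow finds BP_LaserGenerator actors, with the last one checked setting the state.
; State changes send TurnOn/TurnOff messages, but LastValue updates inside the loop, so only the first connected actor receives them.
; Construction script displays allowed IDs as text; overlap-event binding is unused.
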(event Custom|BeginOverlap
  (params (OverlappedComponent :type Primitive%20Component%20Object%20Reference) (OtherActor :type Actor%20Object%20Reference) (OtherComp :type Primitive%20Component%20Object%20Reference) (OtherBodyIndex :type Integer) (bFromSweep :type Boolean) (SweepResult :type Hit%20Result%20Structure%20%28by%20ref%29))
  ;[1 1 1] Comment
  (Development|PrintString (Utilities|String|Append (Utilities|GetDisplayName OtherActor) (Utilities|GetDisplayName OtherComp) "\\") true true "(R=1.000000,G=0.000000,B=0.086574,A=1.000000)"))

(event Custom|EndOverlap
  (params (OverlappedComponent :type Primitive%20Component%20Object%20Reference) (OtherActor :type Actor%20Object%20Reference) (OtherComp :type Primitive%20Component%20Object%20Reference) (OtherBodyIndex :type Integer))
  ;[1 1 1] Comment
  (Development|PrintString (Utilities|String|Append (Utilities|GetDisplayName OtherActor) (Utilities|GetDisplayName OtherComp) "\\") true true "(R=1.000000,G=0.000000,B=0.029677,A=1.000000)"))

(event EventBeginPlay
  ;[1 1 1] Comment
)

(event EventTick
  (params (DeltaSeconds :type Float%20%28single-precision%29))
  (bind _defaultsceneroot (Variables|Default|GetDefaultSceneRoot))
  (bind _arrowup (Variables|Default|GetArrowUp))
  (bind _returnvalue (Transformation|GetWorldLocation _arrowup))
  (bind _returnvalue_2 (Math|Vector|GetUpVector _defaultsceneroot))
  (bind _returnvalue_3 (* _returnvalue_2 1e+01))
  (bind _returnvalue_4 (+ _returnvalue _returnvalue_3))
  (bind _outactors (Collision|BoxOverlapActors _returnvalue_4 "10.000000,10.000000,20.000000" (Utilities|Array|MakeArray "ObjectTypeQuery1" "ObjectTypeQuery2" "ObjectTypeQuery4") "/Game/Items/Lasery/BP_LaserGenerator.BP_LaserGenerator_C" :!class /Script/Engine.KismetSystemLibrary))
  (Utilities|FlowControl|Sequence
    (:then_0
      (Rendering|Debug|DrawDebugBox _returnvalue_4 "10.000000,10.000000,20.000000" "(R=1.000000,G=0.000000,B=0.704562,A=1.000000)" (Transformation|GetActorRotation) 0.0 1.0))
    (:then_1
      (Variables|Default|SetCurValue false))
    (:then_2
      (for _array_element _outactors
        (bind _asbp_laser_generator (Utilities|Casting|CastToBP_LaserGenerator _array_element)
          (:then
            (Variables|Default|SetCurValue (Utilities|Array|ContainsItem (Variables|Default|GetLaserIdAllowed) (Variables|/Game/Items/Lasery/BP_LaserGenerator.BP_LaserGenerator_C|GetlaserId _asbp_laser_generator))))
          (:CastFailed
            (Development|PrintString "casto bp_laseregenrator failed in bp_laserreciever")))))
    (:then_3
      (for _array_element_2 (Variables|Default|GetConnectedActors)
        (if (!= (Variables|Default|GetLastValue) (Variables|Default|GetCurValue))
          (if (Variables|Default|GetCurValue)
            (Class|BPIActivatedbyLaserReciever|Turnon(Message) _array_element_2)
            (Variables|Default|SetLastValue true)
            (else
              (Class|BPIActivatedbyLaserReciever|TurnOff(Message) _array_element_2)
              (Variables|Default|SetLastValue false))))))))

(fn ConstructionScript
  (for _array_element (Variables|Default|GetLaserIdAllowed)
    (LocalVariables|Setstring (Utilities|String|Append (LocalVariables|Getstring) (Utilities|String|ToString(Name) _array_element))))
  (Rendering|Components|TextRender|SetText (Variables|Default|GetTextRender) (Utilities|Text|ToText(String) (LocalVariables|Getstring))))