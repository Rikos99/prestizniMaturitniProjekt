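; BP_LaserDvere is a door from the laser item set that slides open or closed when switched on or off.
; Turnon plays a timeline that lerps the Dvere component's relative location between the StartArrow and EndArrow components, which act as placeable endpoints.
; TurnOff reverses the same timeline; the Blueprint contains no trigger logic, only these two events.
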(event EventBeginPlay)

(event EventTurnOff
  (bind _startarrow (Variables|Default|GetstartArrow))
  (bind _endarrow (Variables|Default|GetendArrow))
  (bind _relativelocation (Variables|/Script/Engine.SceneComponent|GetRelativeLocation _endarrow))
  (bind _relativelocation_2 (Variables|/Script/Engine.SceneComponent|GetRelativeLocation _startarrow))
  (bind _newtrack_0 (Timeline|Timeline Reverse)
    (:Update
      (Transformation|SetRelativeLocation (Variables|Default|Getdvere) (Math|Vector|MakeVector (Math|Float|Lerp (.x _relativelocation_2) (.x _relativelocation) _newtrack_0) (Math|Float|Lerp (.y _relativelocation_2) (.y _relativelocation) _newtrack_0) (Math|Float|Lerp (.z _relativelocation_2) (.z _relativelocation) _newtrack_0)) false false))))

(event EventTurnon
  (bind _startarrow (Variables|Default|GetstartArrow))
  (bind _endarrow (Variables|Default|GetendArrow))
  (bind _relativelocation (Variables|/Script/Engine.SceneComponent|GetRelativeLocation _endarrow))
  (bind _relativelocation_2 (Variables|/Script/Engine.SceneComponent|GetRelativeLocation _startarrow))
  (bind _newtrack_0 (Timeline|Timeline Play)
    (:Update
      (Transformation|SetRelativeLocation (Variables|Default|Getdvere) (Math|Vector|MakeVector (Math|Float|Lerp (.x _relativelocation_2) (.x _relativelocation) _newtrack_0) (Math|Float|Lerp (.y _relativelocation_2) (.y _relativelocation) _newtrack_0) (Math|Float|Lerp (.z _relativelocation_2) (.z _relativelocation) _newtrack_0)) false false))))

(fn ConstructionScript)