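; Measuring water container that models displacement by BP_ItemParent items, showing its volume on a widget.
; It starts full at a capacity derived from scene scale, and the widget's refill event tops it up.
; Overlaps add each item's "volume" attribute, clamped at capacity, and track it by name; exits subtract it and disable the item's collision.
; Each change rescales and repositions the water and updates the readout.
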(event OnComponentBeginOverlap(water)
  (params (OverlappedComponent :type Primitive%20Component%20Object%20Reference) (OtherActor :type Actor%20Object%20Reference) (OtherComp :type Primitive%20Component%20Object%20Reference) (OtherBodyIndex :type Integer) (bFromSweep :type Boolean) (SweepResult :type Hit%20Result%20Structure%20%28by%20ref%29))
  ;[1 1 1] Comment
  (if (Utilities|ClassIsChildOf (Utilities|GetClass OtherActor) "/Game/Items/BP_ItemParent.BP_ItemParent_C")
    (CallFunction|WhenObjectinWater OtherActor)
    (Utilities|FlowControl|Delay 0.2)))

(event OnComponentEndOverlap(water)
  (params (OverlappedComponent :type Primitive%20Component%20Object%20Reference) (OtherActor :type Actor%20Object%20Reference) (OtherComp :type Primitive%20Component%20Object%20Reference) (OtherBodyIndex :type Integer))
  ;[1 1 1] Comment
  (if (Utilities|ClassIsChildOf (Utilities|GetClass OtherActor) "/Game/Items/BP_ItemParent.BP_ItemParent_C")
    (Collision|SetActorEnableCollision OtherActor false)
    (CallFunction|WhenObjectOutOfWater (Utilities|GetObjectName OtherActor))))

(event Custom|RefillWater
  (CallFunction|AddWaterVolumeto (- (Variables|Default|GetMaxVolume) (Variables|Default|GetWaterVolume))))

(event EventBeginPlay
  (bind _watešrscene (Variables|Default|GetwatešrScene))
  (bind _relativescale3d (Variables|/Script/Engine.SceneComponent|GetRelativeScale3D _watešrscene))
  (Utilities|FlowControl|Sequence
    (:then_0
      (bind _returnvalue (UserInterface|CreateWidget "/Game/Items/Cube/WBP_NadobaVody.WBP_NadobaVody_C"))
      (Variables|Default|SetwidgetRef _returnvalue)
      (UserInterface|SetWidget (Variables|Default|GetWidget) _returnvalue))
    (:then_1
      (EventDispatchers|BindEventtoRefillWater (Variables|Default|GetwidgetRef) (delegate Custom|RefillWater)))
    (:then_3
      (bind _output_get (Variables|Default|SetMaxVolume (* (.x _relativescale3d) (.y _relativescale3d) (.z _relativescale3d))))
      (CallFunction|AddWaterVolumeto _output_get))))

(fn ConstructionScript)

(fn AddWaterVolumeto
  (params (addWaterVolume :type Float%20%28double-precision%29))
  (bind _watešrscene (Variables|Default|GetwatešrScene))
  (bind _relativelocation (Variables|/Script/Engine.SceneComponent|GetRelativeLocation _watešrscene))
  (Variables|Default|SetWaterVolume (+ addWaterVolume (Variables|Default|GetWaterVolume)))
  (Utilities|FlowControl|Sequence
    (:then_0
      (if (> (Variables|Default|GetWaterVolume) (Variables|Default|GetMaxVolume))
        (Variables|Default|SetWaterVolume (Variables|Default|GetMaxVolume))))
    (:then_1
      (Transformation|SetRelativeScale3D (Variables|Default|Getwater) (Math|Vector|MakeVector 1.0 1.0 (/ (Variables|Default|GetWaterVolume) (Variables|Default|GetMaxVolume))))
      (Transformation|SetRelativeLocation _watešrscene (Math|Vector|MakeVector (.x _relativelocation) (.y _relativelocation) (/ (* (/ (Variables|Default|GetWaterVolume) (Variables|Default|GetMaxVolume)) 1e+02) 2.0)) false false))
    (:then_2
      (Variables|/Script/UMG.TextBlock|SetText (Variables|/Game/Items/Cube/WBP_NadobaVody.WBP_NadobaVody_C|GetVolumeTextBlock (Variables|Default|GetwidgetRef)) (Utilities|Text|ToText(String) (Utilities|String|Append (Utilities|String|ToString(Float) (Variables|Default|GetWaterVolume)) "  out of  " (Utilities|String|ToString(Float) (Variables|Default|GetMaxVolume)) " m^3"))))))

(fn WhenObjectinWater
  (params (OtherActor :type Actor%20Object%20Reference))
  (bind _asbp_item_parent (Utilities|Casting|CastToBP_ItemParent OtherActor)
    (:then
      (Utilities|Map|Add (Variables|Default|GetItemsInWater) (Utilities|GetObjectName _asbp_item_parent) (Math|Conversions|ToFloat(Integer) (.Value (Utilities|Map|Find (Variables|/Game/Items/BP_ItemParent.BP_ItemParent_C|GetItemAtributes _asbp_item_parent) "volume"))))
      (CallFunction|AddWaterVolumeto (Math|Conversions|ToFloat(Integer) (.Value (Utilities|Map|Find (Variables|/Game/Items/BP_ItemParent.BP_ItemParent_C|GetItemAtributes _asbp_item_parent) "volume")))))
    (:CastFailed
      (Development|PrintString "cast to bp_itemaprent in bp_nadobaVody failed"))))

(fn VypsatItemsinWater
  (Development|PrintString "ITEMY VE VODE")
  (Development|PrintString (Utilities|String|Append "aktualni volume: " (Utilities|String|ToString(Float) (Variables|Default|GetWaterVolume))))
  (bind _keys (Utilities|Map|Keys (Variables|Default|GetItemsInWater)))
  (for (_array_element _array_index) _keys
    (Development|PrintString (Utilities|String|Append (Utilities|String|ToString(Integer) _array_index) ". " _array_element " - " (Utilities|String|ToString(Float) (.Value (Utilities|Map|Find (Variables|Default|GetItemsInWater) _array_element)))))))

(fn WhenObjectOutOfWater
  (params (actorObjectName :type String))
  (bind _itemsinwater (Variables|Default|GetItemsInWater))
  (bind (_value _returnvalue) (Utilities|Map|Find _itemsinwater actorObjectName))
  (if _returnvalue
    (CallFunction|AddWaterVolumeto (* _value -1.0))
    (Utilities|Map|Remove (Variables|Default|GetItemsInWater) actorObjectName)
    (Development|PrintString "REMOVED")))