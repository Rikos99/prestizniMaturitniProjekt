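; BP_NemaBarikada is a resizable barrier that plays a dialogue line when the player runs into it.
; The construction script sizes the Barrier box from depth, width and height variables (Hloubka, Sirka, Vyska) and raises it to rest on the actor origin.
; A slightly larger Trigger box detects player overlap and runs BPDialogueComponent with the NemaBarikada row from Hlasky_DataTable.
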(event OnComponentBeginOverlap(Trigger)
  (params (OverlappedComponent :type Primitive%20Component%20Object%20Reference) (OtherActor :type Actor%20Object%20Reference) (OtherComp :type Primitive%20Component%20Object%20Reference) (OtherBodyIndex :type Integer) (bFromSweep :type Boolean) (SweepResult :type Hit%20Result%20Structure%20%28by%20ref%29))
  (bind _bp_dialoguecomponent (Variables|Default|GetBP_DialogueComponent))
  (if (== OtherActor (Game|GetPlayerCharacter 0))
    (Default|SetNewVariables _bp_dialoguecomponent "NemaBarikada" "/Game/UI/Dialogue/Hlasky_DataTable.Hlasky_DataTable" false "" 0 "NewEnumerator5")
    (Default|Interact _bp_dialoguecomponent)))

(event EventBeginPlay)

(event Collision|EventActorBeginOverlap
  (params (OtherActor :type Actor%20Object%20Reference)))

(event EventTick
  (params (DeltaSeconds :type Float%20%28single-precision%29)))

(fn ConstructionScript
  (bind _barrier (Variables|Default|GetBarrier))
  (bind _trigger (Variables|Default|GetTrigger))
  (bind _vyska (Variables|Default|GetVyska))
  (bind _sirka (Variables|Default|GetSirka))
  (bind _hloubka (Variables|Default|GetHloubka))
  (bind _returnvalue (Math|Vector|MakeVector _hloubka _sirka _vyska))
  (Components|Box|SetBoxExtent _barrier _returnvalue true)
  (Transformation|SetRelativeLocation _barrier (Math|Vector|MakeVector 0.0 0.0 (Variables|Default|GetVyska)) false false)
  (Components|Box|SetBoxExtent _trigger (+ _returnvalue "10.000000,10.000000,10.000000") true)
  (Transformation|SetRelativeLocation _trigger (Math|Vector|MakeVector 0.0 0.0 (Variables|Default|GetVyska)) false false))