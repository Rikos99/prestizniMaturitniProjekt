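; BP_Keycard is a keycard item whose mesh is tinted according to its Color attribute.
; Its construction script runs the parent's logic, then calls OnSpawn.
; OnSpawn reads Color from the item attributes and, if it converts to a valid color, creates a dynamic instance of MI_klic on the static mesh and sets its Color Tint parameter.
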(fn ConstructionScript
  (|CallParentFunction)
  (CallFunction|OnSpawn))

(fn OnSpawn
  (bind _itematributes (Variables|Default|GetItemAtributes))
  (bind (_value _returnvalue) (Utilities|Map|Find _itematributes "Color"))
  (bind (_outconvertedcolor _outisvalid) (Math|Conversions|ToColor(LinearColor) _value))
  (if (and _returnvalue _outisvalid)
    (bind _returnvalue_2 (Rendering|Material|CreateDynamicMaterialInstance (Variables|Default|GetStaticMesh) 0 "/Game/Materials/MI_klic.MI_klic" "None" :!class /Script/Engine.PrimitiveComponent))
    (Rendering|Material|SetVectorParameterValue _returnvalue_2 "Color Tint" _outconvertedcolor :!class /Script/Engine.MaterialInstanceDynamic)))