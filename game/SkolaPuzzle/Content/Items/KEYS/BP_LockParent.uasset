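; Base lock Blueprint that players interact with using a key item to trigger a linked actor.
; On Interact while locked, it checks that the active inventory item matches TypeOfKey, then compares its "keyValue" attribute to KeyValue.
; It sends the result to CallActorOnInteract through BPI_OnLockUsed, then marks itself unlocked even on a mismatch.
; VisualUpdateOnUnlocked is an empty hook called afterward; debug prints report outcomes and setup errors.
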(event EventInteract
  (params (inventory :type BPAC%20Inventory%20Object%20Reference) (hitComponent :type Primitive%20Component%20Object%20Reference))
  (bind _inventorymap (Variables|/Game/Player/BPAC_Inventory.BPAC_Inventory_C|GetInventoryMap inventory))
  (bind _activeslotindex (Variables|/Game/Player/BPAC_Inventory.BPAC_Inventory_C|GetActiveSlotIndex inventory))
  (bind _keyvalue (Variables|Default|GetkeyValue))
  (bind (_value _returnvalue) (Utilities|Map|Find _inventorymap _activeslotindex))
  (bind (_objectname _slotimage _class _atributes) (Utilities|Struct|BreakSt_Item _value))
  (bind _value_2 (Utilities|Map|Find _atributes "keyValue"))
  (bind _returnvalue_2 (Utilities|Enum|Equal(Enum) _value_2 _keyvalue))
  ;[0.15 0.15 0.15 0.5] jestlize jeste neni odemceny
  (if (== (Variables|Default|Getunlocked) false)
    (if _returnvalue
      ;[0.15 0.15 0.15 0.5] je objekt v ruce klic?
      (if (== _class (Variables|Default|GettypeOfKey))
        ;[0.15 0.15 0.15 0.5] ma bp_lock validniho actora, ktereho odemyka
        (if (Utilities|IsValid (Variables|Default|GetcallActorOnInteract))
          ;[0.15 0.15 0.15 0.5] ma callActorOnInteract sprany interface?
          (if (Utilities|DoesObjectImplementInterface (Variables|Default|GetcallActorOnInteract) "/Game/Items/KEYS/BPI_OnLockUsed.BPI_OnLockUsed_C")
            (Class|BPIonLockUsed|OnLockUsed(Message) (Variables|Default|GetcallActorOnInteract) _returnvalue_2)
            (Development|PrintString (Utilities|String|SelectString "ZAMEK OTEVREN" "ZAMEK SE NEPODARIL OTEVRIT" _returnvalue_2))
            (Variables|Default|Setunlocked true)
            (CallFunction|VisualUpdateonUnlocked)
            (else
              ;[0.15 0.15 0.15 0.5] Comment
              (Development|PrintString (Utilities|String|Append (Utilities|GetObjectName self) ": jeho interact actor nema  INTERFACE"))))
          (else
            ;[0.15 0.15 0.15 0.5] Comment
            (Development|PrintString (Utilities|String|Append (Utilities|GetObjectName self) ": NENI NASTAVENY ACTOR SE KTERYM ITERAGUJE"))))
        (else
          (Development|PrintString "spatny item v ruce"))))))

(fn ConstructionScript)

(fn VisualUpdateonUnlocked)