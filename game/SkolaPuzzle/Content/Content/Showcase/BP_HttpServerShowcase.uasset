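; BP_HttpServerShowcase is a demo HTTP server Blueprint that exposes web endpoints to the game.
; BindRoutes registers a GET route, /showcase, returning an inline HTML placeholder page, and a POST route, /spawnCube.
; The POST handler maps the "color" query parameter through the Color map, broadcasts the result via the OnSpawnCube dispatcher, and replies OK, leaving spawning to listeners.
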(event EventBindRoutes
  (Class|SimpleHttpServer|BindRoute "/showcase" "GET" (EventDispatchers|CreateEvent :!event GetShowcase))
  (Class|SimpleHttpServer|BindRoute "/spawnCube" "POST" (EventDispatchers|CreateEvent :!event PostSpawnCube)))

(fn GetShowcase
  (params (HttpServerRequest :type Native%20Http%20Server%20Request%20Structure))
  (Development|PrintString "hiii")
  (bind _returnvalue (Class|SimpleHttpServer|MakeResponse "<!DOCTYPE html> 
<html lang=\"en\"> 
<head> 
  <meta charset=\"UTF-8\"> 
  <meta name=\"viewport\" content=\"width=device-width, initial-scale=1.0\"> 
  <title>POST Request Demo</title> 
  <style> 
    body { font-family: Arial, sans-serif; padding: 20px; } 
    input, button { padding: 10px; margin-top: 10px; } 
    #response { margin-top: 20px; color: green; } 
  </style> 
</head> 
<body> 
hiiii</body> 
</html> 
" "text/html" 200))
  (return _returnvalue))

(fn PostSpawnCube
  (params (HttpServerRequest :type Native%20Http%20Server%20Request%20Structure))
  (Default|CallOnSpawnCube (.Value (Utilities|Map|Find (Variables|Default|GetColor) (.Value (Utilities|Map|Find (.QueryParams (Utilities|Struct|BreakNativeHttpServerRequest HttpServerRequest)) "color")))))
  (bind _returnvalue (Class|SimpleHttpServer|MakeResponse "OK" "application/json" 200))
  (return _returnvalue))