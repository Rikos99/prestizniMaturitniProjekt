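; BP_R2_Projection is a projection actor that displays a randomly chosen graph image through a widget component.
; BeginPlay fills a Graphs array with two structs, each pairing a texture with a list of viable answers that is currently a blank string.
; ChangeToRandomGraph picks a random entry and sets its texture as the image brush on WBP_R2_Projection.
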(event Custom|ChangeToRandomGraph
  (bind _graphs (Variables|Default|Getgraphs))
  (bind _aswbp_r2_projection (Utilities|Casting|CastToWBP_R2_Projection (UserInterface|GetWidget (Variables|Default|GetWidget))))
  (Class|Image|SetBrush (Variables|/Game/AI_Robots/R2-Grafy/r2_projection/WBP_R2_Projection.WBP_R2_Projection_C|GetImage _aswbp_r2_projection) (Class|WidgetBlueprintLibrary|MakeBrushfromTexture (.image (Utilities|Struct|BreakStruct_FuncGraphs (Utilities|Array|Get(acopy) _graphs (Math|Random|RandomIntegerinRange 0 (- (Utilities|Array|Length _graphs) 1))))))))

(event EventBeginPlay
  (Variables|Default|Setgraphs (Utilities|Array|MakeArray (Utilities|Struct|MakeStruct_FuncGraphs "/Game/AI_Robots/R2-Grafy/graphsImages/graph3.graph3" (Utilities|Array|MakeArray "")) (Utilities|Struct|MakeStruct_FuncGraphs "/Game/AI_Robots/R2-Grafy/graphsImages/graph2.graph2" (Utilities|Array|MakeArray ""))))
  (CallFunction|ChangetoRandomGraph))

(fn ConstructionScript)