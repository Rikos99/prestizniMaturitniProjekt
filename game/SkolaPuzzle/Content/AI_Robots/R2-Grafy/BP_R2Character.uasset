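; R2 robot character that presents a graph quiz puzzle using a projection and a widget.
; On BeginPlay it caches the graph list from BP_GameMode.
; Interact switches the Blackboard State: Idle starts Walking to find a projection actor, Projecting returns to Idle.
; StartPuzzle puts the first graph's question into the R2 interface's quiz template and switches the given projection to that graph.
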(event EventBeginPlay
  (bind _asbp_game_mode (Utilities|Casting|CastToBP_GameMode (Game|GetGameMode)))
  (Variables|Default|SetGraphs (Variables|/Game/BP_GameMode.BP_GameMode_C|GetGraphs _asbp_game_mode)))

(event EventInteract
  (params (inventory :type BPAC%20Inventory%20Object%20Reference) (hitComponent :type Primitive%20Component%20Object%20Reference))
  (switch Utilities|FlowControl|Switch|SwitchonEnum_R2_States (Utilities|Enum|ByteToEnumEnum_R2_States (Class|BlackboardComponent|GetValueasEnum (AI|GetBlackboard 0) (Utilities|Name|MakeLiteralName "State")))
    (:NewEnumerator0
      ;[1 1 1] prepnuti stavu na chozeni (hleda projection actor a jde)
      (AI|Components|Blackboard|SetValueasEnum (AI|GetBlackboard 0) (Utilities|Name|MakeLiteralName "State") (Utilities|Enum|LiteralenumEnum_R2_States "NewEnumerator1")))
    (:NewEnumerator2
      ;[1 1 1] prepnuti stavu na idle (hleda projection actor a jde)
      (AI|Components|Blackboard|SetValueasEnum (AI|GetBlackboard 0) (Utilities|Name|MakeLiteralName "State") (Utilities|Enum|LiteralenumEnum_R2_States "NewEnumerator0")))))

(fn ConstructionScript)

(fn StartPuzzle
  (params (projection :type BP%20R2%20Projection%20Object%20Reference))
  (bind _graphs (Variables|Default|GetGraphs))
  (bind _output (Utilities|Array|Get(acopy) _graphs))
  (Utilities|FlowControl|Sequence
    (:then_0
      (bind _aswbp_r2_interface (Utilities|Casting|CastToWBP_R2_Interface (UserInterface|GetWidget (Variables|Default|GetWidget)))
        (:then
          (Default|ContentChange (Variables|/Game/AI_Robots/R2-Grafy/WBP_R2_Interface.WBP_R2_Interface_C|GetWBP_QuizTemplate _aswbp_r2_interface) (.QuiezQuestion (Utilities|Struct|BreakStruct_FuncGraphs _output))))
        (:CastFailed
          (Development|PrintString "XXXX"))))
    (:then_1
      (Default|ChangetoGraph projection _output))))