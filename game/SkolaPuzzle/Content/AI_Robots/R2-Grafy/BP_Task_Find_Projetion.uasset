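; Behavior tree task for the R2 robot AI that picks one BP_R2_Projection actor and stores it in the blackboard.
; On execute it loops over all projection actors, keeping the one with the smallest squared XY location length, measured from world origin rather than the robot.
; It writes the result to the ClosestProjection key and succeeds, or fails when no projections exist.
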(event EventReceiveExecuteAI
  (params (OwnerController :type AI%20Controller%20Object%20Reference) (ControlledPawn :type Pawn%20Object%20Reference))
  (bind _outactors (Actor|GetAllActorsOfClass "/Game/AI_Robots/R2-Grafy/r2_projection/BP_R2_Projection.BP_R2_Projection_C"))
  (if (> (Utilities|Array|Length _outactors) 0)
    (for _array_element _outactors
      (if (Utilities|IsValid (Variables|Default|GetClosestProjection))
        (if (> (Class|KismetMathLibrary|VSizeXYSquared (Transformation|GetActorLocation (Variables|Default|GetClosestProjection))) (Class|KismetMathLibrary|VSizeXYSquared (Transformation|GetActorLocation _array_element)))
          (Variables|Default|SetClosestProjection _array_element))
        (else
          (Variables|Default|SetClosestProjection _array_element))))
    (AI|Components|Blackboard|SetValueasObject (Class|BTFunctionLibrary|GetOwnersBlackboard) (Utilities|Name|MakeLiteralName "ClosestProjection") (Variables|Default|GetClosestProjection))
    (AI|BehaviorTree|FinishExecute true)
    (else
      (AI|BehaviorTree|FinishExecute false))))