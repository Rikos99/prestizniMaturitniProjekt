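; AI controller for the R3-CERES robot that runs BT_Ceres and feeds perception results into its Blackboard.
; On BeginPlay it also stores an actor of class NewBlueprint as ObjectKey.
; The sight handler sets the player as TargetActor, or clears it on sight loss and requests a short movement prediction.
; The prediction handler writes the predicted position to LastKnownLocation; neither handler is called within this graph.
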(event EventBeginPlay
  (AI|RunBehaviorTree "/Game/AI_Robots/R3-CERES/BT_Ceres.BT_Ceres")
  (bind _returnvalue (Actor|GetActorOfClass "/Game/AI_Robots/R3-CERES/NewBlueprint.NewBlueprint_C"))
  (AI|Components|Blackboard|SetValueasObject (AI|GetBlackboard 0) (Utilities|Name|MakeLiteralName "ObjectKey") _returnvalue))

(fn ConstructionScript)

(fn HandleSightSence
  (params (actor :type Actor%20Object%20Reference) (stim :type AI%20Stimulus%20Structure))
  (bind _returnvalue (Class|AIPerceptionSystem|GetSenseClassforStimulus stim))
  (if (== _returnvalue "/Script/AIModule.AISense_Sight")
    (if (== (Game|GetPlayerCharacter 0) actor)
      (AI|Components|Blackboard|SetValueasObject (Variables|Default|GetBlackboard) (Utilities|Name|MakeLiteralName "TargetActor") (Utilities|SelectObject actor 0 (.bsuccessfullysensed stim)))
      (if (not (.bsuccessfullysensed stim))
        (Class|AISensePrediction|RequestPawnPredictionEvent (Pawn|GetControlledPawn) (Game|GetPlayerCharacter 0) 1.0))
      (else
        (return)))
    (else
      (return))))

(fn HandlePrediction
  (params (stim :type AI%20Stimulus%20Structure))
  (bind _returnvalue (Class|AIPerceptionSystem|GetSenseClassforStimulus stim))
  (if (== _returnvalue "/Script/AIModule.AISense_Prediction")
    (if (.bsuccessfullysensed stim)
      (AI|Components|Blackboard|SetValueasVector (Variables|Default|GetBlackboard) (Utilities|Name|MakeLiteralName "LastKnownLocation") (.stimuluslocation stim)))
    (else
      (return))))