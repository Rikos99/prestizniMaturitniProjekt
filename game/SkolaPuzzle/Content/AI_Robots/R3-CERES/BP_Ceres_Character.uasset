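; BP_Ceres_Character is the CERES robot AI character, which opens doors in its path and drives its behavior through a Blackboard State enum.
; BeginPlay and Interact both set that state to Walking through a helper function.
; A looping half-second timer runs a debug-drawn forward multi-trace and opens any closed, unlocked BP_Dvere it hits.
; An uncalled radius-based door opener and disconnected dialogue nodes remain in the graph.
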(event Custom|CustomEvent
  (bind _outactors (Actor|GetAllActorsOfClass "/Game/Items/BP_Dvere.BP_Dvere_C"))
  (bind _array_element (Utilities|Array|ForEachLoopwithBreak _outactors)
    (:LoopBody
      (if (< (Math|Float|Absolute(Float) (Math|Vector|VectorLength (- (Transformation|GetActorLocation _array_element) (Transformation|GetActorLocation)))) 5e+02)
        (if (and (Variables|/Game/Items/BP_Dvere.BP_Dvere_C|GetClosed _array_element) (Variables|/Game/Items/BP_Dvere.BP_Dvere_C|GetUnlocked _array_element))
          (Default|OpenDoor _array_element))))))

(event Custom|CustomEvent_0
  (bind _robotprojektor (Variables|Default|GetrobotProjektor))
  (bind _returnvalue (Transformation|GetWorldLocation _robotprojektor))
  (bind _outhits (Collision|MultiLineTraceByChannel _returnvalue (+ _returnvalue (* (Transformation|GetActorForwardVector) 5e+02)) "TraceTypeQuery1" false 0 "ForDuration" true "(R=1.000000,G=0.000000,B=0.000000,A=1.000000)" "(R=0.000000,G=1.000000,B=0.000000,A=1.000000)" 1.0))
  (for _array_element _outhits
    (Development|PrintString (Utilities|GetDisplayName (.HitActor (Collision|BreakHitResult _array_element))))
    (if (== (Utilities|GetClass (.HitActor (Collision|BreakHitResult _array_element))) "/Game/Items/BP_Dvere.BP_Dvere_C")
      (bind _asbp_dvere (Utilities|Casting|CastToBP_Dvere (.HitActor (Collision|BreakHitResult _array_element))))
      (Development|PrintString (Utilities|String|ToString(Boolean) (Variables|/Game/Items/BP_Dvere.BP_Dvere_C|GetIsOpening _asbp_dvere)))
      (if (Math|Boolean|ANDBoolean (Variables|/Game/Items/BP_Dvere.BP_Dvere_C|GetClosed _asbp_dvere) (Variables|/Game/Items/BP_Dvere.BP_Dvere_C|GetUnlocked _asbp_dvere) (not (Variables|/Game/Items/BP_Dvere.BP_Dvere_C|GetIsOpening _asbp_dvere)))
        (Default|OpenDoor _asbp_dvere)))))

(event EventBeginPlay
  (Utilities|Time|SetTimerbyEvent (delegate Custom|CustomEvent_0) 0.5 true)
  (Development|PrintString "begin")
  (CallFunction|SetBBState "NewEnumerator1"))

(event EventInteract
  (params (inventory :type BPAC%20Inventory%20Object%20Reference) (hitComponent :type Primitive%20Component%20Object%20Reference))
  (CallFunction|SetBBState "NewEnumerator1"))

(fn ConstructionScript)

(fn SetBBState
  (params (state :type Enum_Ceres_States%20Enum :default "NewEnumerator0"))
  (AI|Components|Blackboard|SetValueasEnum (AI|GetBlackboard 0) (Utilities|Name|MakeLiteralName "State") state))

(fn GetBBState
  (return (Utilities|Enum|ByteToEnumEnum_Ceres_States (Class|BlackboardComponent|GetValueasEnum (AI|GetBlackboard 0) (Utilities|Name|MakeLiteralName "State")))))