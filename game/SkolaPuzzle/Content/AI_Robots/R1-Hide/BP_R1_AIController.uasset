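; AI controller for the R1 hiding robot that runs BT_R1 and starts with sight sensing disabled.
; When perception updates on the player, it sets the Blackboard State enum and disables sight again.
; HandlePrediction can store a successful prediction stimulus as LastKnownLocation, but nothing here calls it.
; HandleSightSence is an empty stub.
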(event OnTargetPerceptionUpdated(AIPerception)
  (params (Actor :type Actor%20Object%20Reference) (Stimulus :type AI%20Stimulus%20Structure))
  (if (== (Game|GetPlayerCharacter 0) Actor)
    (AI|Components|Blackboard|SetValueasEnum (Variables|Default|GetBlackboard) (Utilities|Name|MakeLiteralName "State") (Utilities|Enum|LiteralenumEnum_R1Sates "NewEnumerator2"))
    (Class|AIPerceptionComponent|SetSenseEnabled (Variables|Default|GetAIPerception) "/Script/AIModule.AISense_Sight" false)))

(event EventBeginPlay
  (AI|RunBehaviorTree "/Game/AI_Robots/R1-Hide/BT_R1.BT_R1")
  (Class|AIPerceptionComponent|SetSenseEnabled (Variables|Default|GetAIPerception) "/Script/AIModule.AISense_Sight" false))

(fn ConstructionScript)

(fn HandleSightSence
  (params (actor :type Actor%20Object%20Reference) (stim :type AI%20Stimulus%20Structure)))

(fn HandlePrediction
  (params (stim :type AI%20Stimulus%20Structure))
  (bind _returnvalue (Class|AIPerceptionSystem|GetSenseClassforStimulus stim))
  (if (== _returnvalue "/Script/AIModule.AISense_Prediction")
    (if (.bsuccessfullysensed stim)
      (AI|Components|Blackboard|SetValueasVector (Variables|Default|GetBlackboard) (Utilities|Name|MakeLiteralName "LastKnownLocation") (.stimuluslocation stim)))
    (else
      (return))))