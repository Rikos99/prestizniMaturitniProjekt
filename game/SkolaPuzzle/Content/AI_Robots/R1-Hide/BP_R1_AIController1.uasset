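; AI controller for the R1 robot that runs behavior tree BT_R1 and feeds it perception data about the player.
; Sight updates for player character 0 set the TargetActor blackboard key, clearing it when sight is lost.
; Losing sight also requests a short prediction of the player's movement, whose successful stimulus writes the predicted position to LastKnownLocation.
; Every perception update also prints a debug string.
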(event OnTargetPerceptionUpdated(AIPerception)
  (params (Actor :type Actor%20Object%20Reference) (Stimulus :type AI%20Stimulus%20Structure))
  (Development|PrintString "Hello")
  (CallFunction|HandleSightSence Actor Stimulus)
  (CallFunction|HandlePrediction Stimulus))

(event EventBeginPlay
  (AI|RunBehaviorTree "/Game/AI_Robots/R1-Hide/BT_R1.BT_R1"))

(fn ConstructionScript)

(fn HandleSightSence
  (params (actor :type Actor%20Object%20Reference) (stim :type AI%20Stimulus%20Structure))
  (bind _returnvalue (Class|AIPerceptionSystem|GetSenseClassforStimulus stim))
  (if (== _returnvalue "/Script/AIModule.AISense_Sight")
    (if (== (Game|GetPlayerCharacter 0) actor)
      (AI|Components|Blackboard|SetValueasObject (Variables|Default|GetBlackboard) (Utilities|Name|MakeLiteralName "TargetActor") (Utilities|SelectObject actor 0 (.bsuccessfullysensed stim)))
      (if (not (.bsuccessfullysensed stim))
        (Class|AISensePrediction|RequestPawnPredictionEvent (Pawn|GetControlledPawn) (Game|GetPlayerCharacter 0) 1.0))
      (else
        (return)))
    (else
      (return))))

(fn HandlePrediction
  (params (stim :type AI%20Stimulus%20Structure))
  (bind _returnvalue (Class|AIPerceptionSystem|GetSenseClassforStimulus stim))
  (if (== _returnvalue "/Script/AIModule.AISense_Prediction")
    (if (.bsuccessfullysensed stim)
      (AI|Components|Blackboard|SetValueasVector (Variables|Default|GetBlackboard) (Utilities|Name|MakeLiteralName "LastKnownLocation") (.stimuluslocation stim)))
    (else
      (return))))