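; BP_R1Character is the R1 robot AI character, whose behaviour state the Interact event toggles.
; Interact calls OnInteract, which reads the State enum key on the AI blackboard.
; If State holds one specific R1 state it switches to a second, and from any other state it switches to the first.
; The Blueprint holds no other logic, only writing the new state back to the blackboard.
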(event EventInteract
  (params (inventory :type BPAC%20Inventory%20Object%20Reference) (hitComponent :type Primitive%20Component%20Object%20Reference))
  (CallFunction|OnInteract))

(fn ConstructionScript)

(fn OnInteract
  (bind _returnvalue (Utilities|Name|MakeLiteralName "State"))
  (bind _returnvalue_2 (AI|GetBlackboard 0))
  (if (Utilities|Enum|Equal(Enum) (Utilities|Enum|ByteToEnumEnum_R1_Sates (Class|BlackboardComponent|GetValueasEnum (AI|GetBlackboard 0) (Utilities|Name|MakeLiteralName "State"))) (Utilities|Enum|LiteralenumEnum_R1_Sates "NewEnumerator3"))
    (AI|Components|Blackboard|SetValueasEnum _returnvalue_2 _returnvalue (Utilities|Enum|LiteralenumEnum_R1_Sates "NewEnumerator0"))
    (else
      (AI|Components|Blackboard|SetValueasEnum _returnvalue_2 _returnvalue (Utilities|Enum|LiteralenumEnum_R1_Sates "NewEnumerator3")))))