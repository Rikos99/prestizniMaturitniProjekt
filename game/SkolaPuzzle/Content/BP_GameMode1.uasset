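; Game mode Blueprint that fills hardcoded game data when play begins, with no other active logic.
; It builds the in-game computer's app list from window structs that pair names with widgets.
; It also defines tagged quizzes with differing question types and accepted answers, plus graph images paired with quiz questions.
; An item icon map links the cable class to a texture; much of the quiz content looks like Czech test data.
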(event EventBeginPlay
  (Variables|Default|SetAppsOnComputer (Utilities|Array|MakeArray (Utilities|Struct|MakeBPS_Window "Ahooj" "/Game/UI/Computer/WindowsContents/WBP_Ahooj.WBP_Ahooj_C") (Utilities|Struct|MakeBPS_Window "Timer" "/Game/UI/Computer/WindowsContents/WBP_Timer.WBP_Timer_C") (Utilities|Struct|MakeBPS_Window "Usbs" "/Game/UI/Computer/WindowsContents/WBP_Usbs.WBP_Usbs_C")))
  (Variables|Default|Setquizes (Utilities|Array|MakeArray (Utilities|Struct|MakeSt_Quiz "barvicky1" "test kvizu" (Utilities|Array|MakeArray (Utilities|Struct|MakeSt_QuizQuestion "zelena barva v anglicky" (Utilities|Array|MakeArray "yellow" "green" "red") (Utilities|Set|MakeSet 1)) (Utilities|Struct|MakeSt_QuizQuestion "barvikca ruzova" (Utilities|Array|MakeArray "pink" "purple" "green" "pastel pink") (Utilities|Set|MakeSet 0 3) "()" "NewEnumerator2") (Utilities|Struct|MakeSt_QuizQuestion "barvikca vsechny ruzova" (Utilities|Array|MakeArray "pink" "purple" "green" "pastel pink") (Utilities|Set|MakeSet 0 3) "()" "NewEnumerator1")) 2) (Utilities|Struct|MakeSt_Quiz "test1" "barvicky " (Utilities|Array|MakeArray (Utilities|Struct|MakeSt_QuizQuestion "barvikca vsechny ruzova xx" (Utilities|Array|MakeArray "pink" "purple" "green" "pastel pink") (Utilities|Set|MakeSet 0 3) "()" "NewEnumerator2")))))
  (Variables|Default|SetItemIcons (Utilities|Map|MakeMap "/Game/Items/Cable/BP_Cable.BP_Cable_C" "/Game/Textures/a411-stul/a411-stul_DefaultMaterial_OcclusionRoughnessMetallic.a411-stul_DefaultMaterial_OcclusionRoughnessMetallic"))
  (Variables|Default|Setgraphs (Utilities|Array|MakeArray (Utilities|Struct|MakeStruct_FuncGraphs "/Game/AI_Robots/R2-Grafy/graphsImages/graph3.graph3" (Utilities|Struct|MakeSt_QuizQuestion "Jaky je predpis grafu?" (Utilities|Array|MakeArray "prvni " "druha " "treti" "ctvrta") (Utilities|Set|MakeSet 0))))))

(event EventTick
  (params (DeltaSeconds :type Float%20%28single-precision%29)))

(fn ConstructionScript)