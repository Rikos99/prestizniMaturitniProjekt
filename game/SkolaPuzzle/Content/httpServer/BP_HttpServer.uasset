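; BP_HttpServer is an in-engine HTTP server Blueprint that serves test web pages and receives posted text.
; BindRoutes registers GET routes /posttest and /hi and POST route /datasend, with handlers returning responses built by MakeResponse.
; Hello returns static HTML, while POSTTEST serves an inline form whose script posts JSON to localhost /datasend.
; GetPost prints the request body and returns an empty 200, although the page script expects a JSON message.
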(event EventBindRoutes
  (Class|SimpleHttpServer|BindRoute "/posttest" "GET" (EventDispatchers|CreateEvent :!event POSTTEST))
  (Class|SimpleHttpServer|BindRoute "/hi" "GET" (EventDispatchers|CreateEvent :!event Hello))
  (Class|SimpleHttpServer|BindRoute "/datasend" "POST" (EventDispatchers|CreateEvent :!event GetPost)))

(fn Hello
  (params (HttpServerRequest :type Native%20Http%20Server%20Request%20Structure))
  (bind _returnvalue (Class|SimpleHttpServer|MakeResponse "<!DOCTYPE html> 
<html> 
  <head> 
  </head> 
  <body><h1>HIII</h1> 
  </body> 
</html>" "text/html" 200))
  (return _returnvalue))

(fn POSTTEST
  (params (HttpServerRequest :type Native%20Http%20Server%20Request%20Structure))
  (bind _returnvalue (Class|SimpleHttpServer|MakeResponse "<!DOCTYPE html> 
<html lang=\"en\"> 
<head> 
  <meta charset=\"UTF-8\"> 
  <meta name=\"viewport\" content=\"width=device-width, initial-scale=1.0\"> 
  <title>POST Request Demo</title> 
  <style> 
    body { font-family: Arial, sans-serif; padding: 20px; } 
    input, button { padding: 10px; margin-top: 10px; } 
    #response { margin-top: 20px; color: green; } 
  </style> 
</head> 
<body> 
 
  <h1>Send a POST Request</h1> 
   
  <label for=\"userInput\">Enter text:</label> 
  <input type=\"text\" id=\"userInput\" placeholder=\"Type something...\" /> 
  <button onclick=\"sendPostRequest()\">Send</button> 
 
  <div id=\"response\"></div> 
 
  <script> 
    async function sendPostRequest() { 
      const userInput = document.getElementById(\"userInput\").value; 
      const responseDiv = document.getElementById(\"response\"); 
 
      try { 
        const response = await fetch(\"http://127.0.0.1:8080/datasend\", { 
          method: \"POST\", 
          headers: { 
            \"Content-Type\": \"application/json\" 
          }, 
          body: JSON.stringify({ text: userInput }) 
        }); 
         
        if (response.ok) { 
          const responseData = await response.json(); 
          responseDiv.textContent = \"Server response: \" + responseData.message; 
        } else { 
          responseDiv.textContent = \"Error: \" + response.statusText; 
        } 
      } catch (error) { 
        responseDiv.textContent = \"Network error: \" + error.message; 
      } 
    } 
  </script> 
 
</body> 
</html> 
" "text/html" 200))
  (return _returnvalue))

(fn GetPost
  (params (HttpServerRequest :type Native%20Http%20Server%20Request%20Structure))
  (Development|PrintString (.Body (Utilities|Struct|BreakNativeHttpServerRequest HttpServerRequest)))
  (bind _returnvalue (Class|SimpleHttpServer|MakeResponse "" "" 200))
  (return _returnvalue))