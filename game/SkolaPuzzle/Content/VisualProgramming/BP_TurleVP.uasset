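; Interactive turtle-graphics visual programming station with a controller widget, a turtle screen widget and a physical run button.
; On BeginPlay it gives the controller's main canvas references to itself and the turtle screen.
; Interacting with the controller hands its widget to the first-person character's full-widget view.
; The run button animates on press, then, only if the screen's turtle is valid, runs the canvas program and plays a second button-movement timeline.
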(event EventBeginPlay
  (bind _aswbp_vp_main_canvas (Utilities|Casting|CastToWBP_VP_MainCanvas (UserInterface|GetWidget (Variables|Default|GetControllerWidget))))
  (Variables|/Game/VisualProgramming/WBP_VP_MainCanvas.WBP_VP_MainCanvas_C|SetTurtleActor _aswbp_vp_main_canvas self)
  (bind _aswbp_vp_turtle_screen (Utilities|Casting|CastToWBP_VP_TurtleScreen (UserInterface|GetWidget (Variables|Default|GetScreenTurtleWidget))))
  (Variables|/Game/VisualProgramming/WBP_VP_MainCanvas.WBP_VP_MainCanvas_C|SetWbp_vp_TurtleScreen _aswbp_vp_main_canvas _aswbp_vp_turtle_screen))

(event EventInteract
  (params (inventory :type BPAC%20Inventory%20Object%20Reference) (hitComponent :type Primitive%20Component%20Object%20Reference))
  (if (== hitComponent (Variables|Default|GetControllerWidget))
    (bind _asbp_first_person_character (Utilities|Casting|CastToBP_FirstPersonCharacter (Game|GetPlayerCharacter 0)))
    (Default|BeginonWidegtFull _asbp_first_person_character (UserInterface|GetWidget (Variables|Default|GetControllerWidget)))
    (elif (== hitComponent (Variables|Default|GetRunButton))
      (bind _offset (Timeline|Press%20Button PlayFromStart)
        (:Update
          (Transformation|SetRelativeLocation (Variables|Default|GetRunButton) (Math|Vector|MakeVector 0.0 0.0 _offset) false false))
        (:Finished
          (bind _aswbp_vp_main_canvas (Utilities|Casting|CastToWBP_VP_MainCanvas (UserInterface|GetWidget (Variables|Default|GetControllerWidget))))
          (Utilities|IsValid (Variables|/Game/VisualProgramming/WBP_VP_TurtleScreen.WBP_VP_TurtleScreen_C|GetWBP_Turtle (Variables|/Game/VisualProgramming/WBP_VP_MainCanvas.WBP_VP_MainCanvas_C|GetWbp_vp_TurtleScreen _aswbp_vp_main_canvas))
            (:Is%20Valid
              (Default|RunProgram _aswbp_vp_main_canvas)
              (bind _offset_2 (Timeline|Timeline PlayFromStart)
                (:Update
                  (Transformation|SetRelativeLocation (Variables|Default|GetRunButton) (Math|Vector|MakeVector 0.0 0.0 _offset_2) false false))))))))))

(fn ConstructionScript)